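; Inventory/shop preview pawn that displays a modular character and swaps its part meshes by item.
; Hair, top, bottoms, shoes and hand meshes follow Body as master pose, with custom depth on Top and Hair.
; Opening the shop resolves uploaded player items through the game instance and applies their meshes before showing Body; closing hides it.
; Position lookup finds a part's "Scene"-suffixed child component by data-table class name.
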(event Custom|Shop_Defalut
  ;[1 1 1] 구조체에 접근해서
  (bind _returnvalue (Class|PawnPlayer|UploadPlayer))
  (bind _asbp_game_instance_solaseado (Utilities|Casting|CastToBP_GameInstance_Solaseado (Game|GetGameInstance)))
  (for _array_element _returnvalue
    (bind _returnvalue_2 (Class|GameInstanceSolaseado|FindITem _asbp_game_instance_solaseado _array_element))
    ;[1 1 1] 메쉬변경
    (Class|PawnPlayer|ChangeMesh (.classname _returnvalue_2) (.mesh _returnvalue_2)))
  (Rendering|SetVisibility (Variables|Default|GetBody) true true))

(event Custom|ShopClose
  (Rendering|SetVisibility (Variables|Default|GetBody) false true))

(event EventBeginPlay
  (bind _asbp_login_pawn (Utilities|Casting|CastToBP_LoginPawn (Game|Player|GetPlayerPawn 0)))
  ;[1 1 1] 컴포넌트가 가지고 있는 데이터에 접근하기위해
  (Variables|Default|SetBP_ActorComponent_Playfab (Variables|/Game/Project/Pawn/Solaseado/BP_LoginPawn.BP_LoginPawn_C|GetActorComponent_Playfab _asbp_login_pawn)))

(fn ConstructionScript
  (Class|SkinnedMeshComponent|SetMasterPoseComponent (Variables|Default|GetShoes) (Variables|Default|GetBody) false)
  (Rendering|SetRenderCustomDepth (Variables|Default|GetTop) true))

(fn BPSelectPosition
  (params (ClassName :type Integer))
  (bind _asgame_instance_solaseado (Utilities|Casting|CastToGameInstance_Solaseado (Game|GetGameInstance)))
  (bind _returnvalue (Utilities|GetDataTableRow (Utilities|Array|Get(acopy) (Class|GameInstanceSolaseado|GetDataTables _asgame_instance_solaseado) ClassName) "1")
    (:then
      (bind _output_get (Variables|Default|SetDataTable _returnvalue))
      (for _array_element (Actor|GetComponentsByClass "/Script/Engine.SkeletalMeshComponent")
        (if (Utilities|Enum|Equal(Enum) (Utilities|GetObjectName _array_element) (.classname _output_get))
          (for _array_element_2 (Components|GetChildrenComponents _array_element false)
            (if (Utilities|Enum|Equal(Enum) (Utilities|GetObjectName _array_element_2) (Utilities|String|Append (Utilities|GetObjectName _array_element) "Scene"))
              (return true (Transformation|GetWorldLocation _array_element_2))))))
      (return false "0, 0, 0"))))

(fn ChangeScene
  (params (TabNumber :type Integer))
  ;[1 1 1] 아직 내용없음
  (|CallParentFunction TabNumber)
  ;[1 1 1] 전체화면
  (return))

(fn ShopInitBind
  (params (WB_ShopMain :type WB%20Shop%20Main%20Object%20Reference))
  (EventDispatchers|BindEventtoClickDispatcher WB_ShopMain (EventDispatchers|CreateEvent :!event ShopChangeMesh))
  (CallFunction|ShopDefalut))

(fn ShopChangeMesh
  (params (ITemID :type String) (ClassName :type String))
  (bind _asbp_game_instance_solaseado (Utilities|Casting|CastToBP_GameInstance_Solaseado (Game|GetGameInstance)))
  (bind _returnvalue (Class|GameInstanceSolaseado|FindITem _asbp_game_instance_solaseado ITemID))
  (Class|PawnPlayer|ChangeMesh (.classname _returnvalue) (.mesh _returnvalue)))