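; BP_Player is a player pawn built from modular character meshes that share animation through master pose components.
; The construction script chains face and hair parts to Head, and Head and Hand to Body.
; A moveRight input issues one nav-based SimpleMoveToLocation sideways through a DoOnce with no reset, while the mouse wheel adjusts and prints Speed.
; Direct movement, zoom and camera rotation logic is disconnected, and mouse axes do nothing.
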(event Input|AxisEvents|InputAxisMouseWheel
  (params (AxisValue :type Float%20%28single-precision%29))
  (if (!= AxisValue 0.0)
    (bind _output_get (Variables|Default|SetSpeed (+ (Variables|Default|GetSpeed) (* AxisValue 0.1))))
    (Development|PrintString (Utilities|String|ToString(Float) _output_get))))

(event Input|AxisEvents|InputAxismoveRight
  (params (AxisValue :type Float%20%28single-precision%29))
  (if (!= AxisValue 0.0)
    (Utilities|FlowControl|DoOnce false
      (:Completed
        (AI|Navigation|SimpleMovetoLocation (Game|GetPlayerController 0) (+ (Transformation|GetActorLocation) (* (* (Transformation|GetActorRightVector) AxisValue) 46.0)))))))

(event Input|AxisEvents|InputAxisMouseX
  (params (AxisValue :type Float%20%28single-precision%29)))

(event Input|AxisEvents|InputAxisMouseY
  (params (AxisValue :type Float%20%28single-precision%29)))

(fn ConstructionScript
  (Class|SkinnedMeshComponent|SetMasterPoseComponent (Variables|Default|GetEyes) (Variables|Default|GetHead) false)
  (Class|SkinnedMeshComponent|SetMasterPoseComponent (Variables|Default|GetHand) (Variables|Default|GetBody) false))