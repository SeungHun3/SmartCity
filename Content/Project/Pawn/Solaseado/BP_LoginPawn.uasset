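; Player pawn for Solaseado that handles PlayFab device-ID login, character creation and in-game player behavior.
; Its PlayFab component handles account requests, while events relay shop, coin, inventory, nickname and quest updates to GameMode-held widgets.
; A loading counter triggers the GameMode's Photon connection, and stopping movement reports location to Photon.
; It also drives tick-based movement, ABP_Player animation states, spring-arm camera changes and master-pose modular body meshes.
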(event Custom|Test_TargetLength
  (bind _springarm (Variables|Default|GetSpringArm))
  ;[1 0.1976 0.2175] Test_카메라 전환
  (Utilities|FlowControl|MultiGate false true -1
    (:Out%200
      (Variables|Default|SetTest_SaveLength (Variables|/Script/Engine.SpringArmComponent|GetTargetArmLength _springarm))
      (Variables|/Script/Engine.SpringArmComponent|SetTargetArmLength _springarm 4.6e+03))
    (:Out%201
      (Variables|/Script/Engine.SpringArmComponent|SetTargetArmLength _springarm (Variables|Default|GetTest_SaveLength)))))

(event Custom|Update%20Inventory%20Coin
  (params (Coin :type Integer))
  ;[1 1 1] 업데이트할 코인 값 인벤토리로 넘겨주는 함수
  (bind _asgm_solaseado (Utilities|Casting|CastToGM_Solaseado (Game|GetGameMode)))
  (Default|SetCoin (Variables|/Game/Project/World/GM_Solaseado.GM_Solaseado_C|GetWB_MainMenu _asgm_solaseado) (Utilities|String|ToString(Integer) Coin)))

(event Custom|Camera_TimeLine
  (params (SceneLocation :type Vector))
  (bind _springarm (Variables|Default|GetSpringArm))
  ;[1 1 1] 카메라 변경
  (bind _새_트랙_0 (Timeline|TimeLine_Change_Camera PlayFromStart)
    (:Update
      (Transformation|SetWorldLocation _springarm (Math|Vector|Lerp(Vector) (Transformation|GetWorldLocation _springarm) SceneLocation _새_트랙_0) false false))))

(event Custom|Login_CustomID
  ;[1 0.9429 0.2055] 기기 ID 값 이용한 간편 로그인
  (switch string (Game|GetPlatformName)
    (:Windows
      (bind _returnvalue (Class|PawnPlayer|GetLoginDeviceID))
      (Variables|Default|SetPlayfabCustomID _returnvalue))
    (:Android
      (Variables|Default|SetPlayfabCustomID (Class|KismetSystemLibrary|GetDeviceId))))
  (Class|ActorComponentPlayfab|LoginCustom (Variables|Default|GetActorComponent_Playfab) (Variables|Default|GetPlayfabCustomID)))

(event Custom|Check_UserTitleName
  (params (DisplayName :type String))
  ;[1 0.9429 0.2055] Playfab  유저 ID 생성 & 확인
  (Class|ActorComponentPlayfab|UpdateUserTitleName (Variables|Default|GetActorComponent_Playfab) DisplayName))

(event EventInitPlayFabUserTitleData
  (params (bChecker :type Boolean))
  ;[1 1 1] Playfab _ 접속시 캐릭터 생성 여부에 따른 로직
  (if bChecker
    (Development|PrintString "// Playfab _ 기존 캐릭터 새성 성공 .")
    (Class|ActorComponentPlayfab|GetIngamePlayerData (Variables|Default|GetActorComponent_Playfab))
    (else
      (Development|PrintString "// Playfab _ 캐릭터 생성값 확인 :: false")
      ;[1 0.1976 0.2175] 커스터마이징 씬 이동
      ; Login Level 임시 적용 > 커스터마이징 씬으로 활용
      (bind _asgm_solaseado (Utilities|Casting|CastToGM_Solaseado (Game|GetGameMode)))
      (Class|GameModeBaseSolaseado|MoveLevel _asgm_solaseado "Login" true))))

(event EventCustomizingWidgetNameChecker
  (params (bChecker :type Boolean))
  ;[1 1 1] Playfab _ Title User ID 설정
  (if (not bChecker)
    (bind _asgm_solaseado (Utilities|Casting|CastToGM_Solaseado (Game|GetGameMode)))
    (Default|CheckerNickname (Variables|/Game/Project/World/GM_Solaseado.GM_Solaseado_C|GetWB_Create_Nickname _asgm_solaseado) false)))

(event EventBlueprintUpdateEquipmentItem
  (params (InstanceID :type String))
  ;[1 1 1] 장비 바꾸기 성공 후 업데이트
  (bind _asgm_solaseado (Utilities|Casting|CastToGM_Solaseado (Game|GetGameMode)))
  (Default|EquipChange (Variables|/Game/Project/Widget/Menu/WB_MainMenu.WB_MainMenu_C|GetWB_Inventory (Variables|/Game/Project/World/GM_Solaseado.GM_Solaseado_C|GetWB_MainMenu _asgm_solaseado)) InstanceID))

(event EventUpdateDisplayNameEvent
  (params (bChecker :type Boolean))
  ;[1 1 1] Playfab _ Title User ID 설정
  (bind _asgm_solaseado (Utilities|Casting|CastToGM_Solaseado (Game|GetGameMode)))
  (Default|CheckerNickname (Variables|/Game/Project/World/GM_Solaseado.GM_Solaseado_C|GetWB_Create_Nickname _asgm_solaseado) bChecker))

(event EventBlueprintCreateCharacter
  ;[1 1 1] Playfab _ 캐릭터 생성 성공 > 인게임 이동
  (Development|PrintString "// Create Character :: Join Game Room")
  (bind _asgm_solaseado (Utilities|Casting|CastToGM_Solaseado (Game|GetGameMode)))
  ;[1 1 1] 성별 업로드 -> 코스튬 정보 서버 업로드
  ; ->게임 정보 로드 / 포톤 챗 연결 결과로 인게임 레벨로 이동
  (Class|ActorComponentPlayfab|UploadMyCustom (Variables|Default|GetActorComponent_Playfab) "Create_Grant" "GrantItems" (Variables|/Script/Test_LidarSample.Widget_Customizing|GetITemIDs (Variables|/Script/Test_LidarSample.PlayerState_Solaseado|GetWidget_Customizing (Class|GameModeBaseSolaseado|GetPlayerStateSolaseado _asgm_solaseado)))))

(event EventCheckGetIngameLoadingCount
  (bind _check_loadingcount (Variables|Default|GetCheck_LoadingCount))
  ;[1 1 1] Test _ Playfab Loading Count
  (Math|Integer|IncrementInt _check_loadingcount
    (:%20%20
      (if (>= _check_loadingcount (Variables|Default|GetTest_LoadingCount))
        ;[1 1 1] // PhotonCloud 접속 성공시 인게임 로직 접속
        ; // Photon, Photon Chat, Photon Voice 동시 접속
        (CallFunction|ConnectPhotonAll)))))

(event EventBlueprintAddInventoryItem
  (params (item :type Itemproperty%20Structure))
  (bind (_itemid _iteminstanceid _itemclass) (Utilities|Struct|BreakItemproperty item))
  ;[1 1 1] 구매한 아이템 슬롯 추가를 위해 값을 넘겨줌
  (bind _asgm_solaseado (Utilities|Casting|CastToGM_Solaseado (Game|GetGameMode)))
  (Default|PurchaseItemAddList (Variables|/Game/Project/Widget/Menu/WB_MainMenu.WB_MainMenu_C|GetWB_Inventory (Variables|/Game/Project/World/GM_Solaseado.GM_Solaseado_C|GetWB_MainMenu _asgm_solaseado)) _itemid _iteminstanceid _itemclass)
  (Default|PurchasedItemInfo (Variables|/Game/Project/Widget/Menu/WB_MainMenu.WB_MainMenu_C|GetShopMain (Variables|/Game/Project/World/GM_Solaseado.GM_Solaseado_C|GetWB_MainMenu _asgm_solaseado)) _itemid _iteminstanceid _itemclass))

(event EventUpdateStore
  (params (ShopDatas :type Array%20of%20I%20Tem%20Info%20Structures))
  ;[1 1 1] 상점정보 업데이트 + coin 정보 최신화
  (bind _shopmain (Utilities|GetShopWidget)
    (:Is%20Valid
      (Default|UpdateShopItems _shopmain ShopDatas))))

(event EventUpdateInventory
  ;[1 1 1] // 인벤토리 정보 수정 :: 코인
  (bind _asgm_solaseado (Utilities|Casting|CastToGM_Solaseado (Game|GetGameMode)))
  (Utilities|IsValid (Variables|/Game/Project/World/GM_Solaseado.GM_Solaseado_C|GetWB_MainMenu _asgm_solaseado)
    (:Is%20Valid
      (Default|SetInventoryCoin (Variables|/Game/Project/Widget/Menu/WB_MainMenu.WB_MainMenu_C|GetWB_Inventory (Variables|/Game/Project/World/GM_Solaseado.GM_Solaseado_C|GetWB_MainMenu _asgm_solaseado)) (Variables|Default|GetVirtualCoin)))))

(event EventCoinUpdate
  (params (coin :type Integer))
  ;[1 1 1] 상점정보 업데이트 + coin 정보 최신화
  (bind _shopmain (Utilities|GetShopWidget)
    (:Is%20Valid
      (Default|UpdateMyCoin _shopmain coin)
      ;[1 1 1] Inventory에 있는 Coin도 업데이트
      (CallFunction|UpdateInventoryCoin coin))))

(event EventChangeAnim
  (params (animstate :type enum_PlayerAnimationState%20Enum :default "Error"))
  ;[1 1 1] 서버에서 받아온 데이터-> AnimInstance에 전달
  (bind _asabp_player (Utilities|Casting|CastToABP_Player (Components|SkeletalMesh|GetAnimInstance (Variables|Default|GetBody))))
  (Variables|/Game/Project/Skeleton/anim/anim_body/ABP_Player.ABP_Player_C|SetBP_AnimState _asabp_player animstate))

(event EventPawnMove
  (params (Loc :type Vector :default "0, 0, 0"))
  (Variables|Default|SetLoc Loc)
  (Variables|Default|SetIsMove true)
  (bind _asabp_player (Utilities|Casting|CastToABP_Player (Components|SkeletalMesh|GetAnimInstance (Variables|Default|GetBody))))
  (Variables|/Game/Project/Skeleton/anim/anim_body/ABP_Player.ABP_Player_C|SetBP_AnimState _asabp_player "Walk"))

(event EventPawnStopMove
  (Variables|Default|SetIsMove false)
  (bind _asgm_solaseado (Utilities|Casting|CastToGM_Solaseado (Game|GetGameMode)))
  (Utilities|IsValid (Variables|/Script/Test_LidarSample.GameModeBase_Solaseado|GetPhotonCloud _asgm_solaseado)
    (:Is%20Valid
      (Class|ActorSolaseadoPhoton|PhotonFinish (Variables|/Script/Test_LidarSample.GameModeBase_Solaseado|GetPhotonCloud _asgm_solaseado) (Transformation|GetActorLocation))
      (bind _asabp_player (Utilities|Casting|CastToABP_Player (Components|SkeletalMesh|GetAnimInstance (Variables|Default|GetBody))))
      (Variables|/Game/Project/Skeleton/anim/anim_body/ABP_Player.ABP_Player_C|SetBP_AnimState _asabp_player "Idle"))))

(event EventTick
  (params (DeltaSeconds :type Float%20%28single-precision%29))
  (bind _loc (Variables|Default|GetLoc))
  (if (Variables|Default|GetIsMove)
    (Transformation|AddWorldOffset (Variables|Default|GetRoot) (* _loc (* (Variables|Default|GetSpeed) (/ 3e+01 (/ 1.0 DeltaSeconds)))) false false)
    (Transformation|SetActorRotation (Math|Rotator|Lerp(Rotator) (Transformation|GetActorRotation) (Math|Conversions|RotationFromXVector _loc) 0.05 true))))

(event Custom|QuestCurrentTableStart
  (params (DataTable :type Data%20Table%20Object%20Reference))
  (bind _asgm_solaseado (Utilities|Casting|CastToGM_Solaseado (Game|GetGameMode)))
  (Variables|/Game/Project/Widget/Popup/WB_DialogueSystem.WB_DialogueSystem_C|SetQuestTable (Variables|/Game/Project/Widget/Menu/WB_MainMenu.WB_MainMenu_C|GetWB_DialogueSystem (Variables|/Game/Project/World/GM_Solaseado.GM_Solaseado_C|GetWB_MainMenu _asgm_solaseado)) DataTable)
  (Default|AddDialogueBox (Variables|/Game/Project/Widget/Menu/WB_MainMenu.WB_MainMenu_C|GetWB_DialogueSystem (Variables|/Game/Project/World/GM_Solaseado.GM_Solaseado_C|GetWB_MainMenu _asgm_solaseado)) DataTable))

(event EventQuestDrop
  (params (QuestName :type String))
  (Development|PrintString (Utilities|String|Append QuestName "__Drop") true true "(R=1.000000,G=0.006201,B=0.000000,A=1.000000)" 1e+01))

(event EventQuestStart
  (params (PlayQuest :type Quest%20Info%20Structure))
  (bind (_quest_name _quest_step _isfinished _questtable) (Utilities|Struct|BreakQuest_Info PlayQuest))
  (Development|PrintString (Utilities|String|Append _quest_name "__Start"))
  (CallFunction|QuestCurrentTableStart _questtable))

(event EventQuestNext
  (params (QuestInfo :type Quest%20Info%20Structure%20%28by%20ref%29))
  (bind (_quest_name _quest_step _isfinished _questtable) (Utilities|Struct|BreakQuest_Info QuestInfo))
  (Development|PrintString (Utilities|String|Append _quest_name "__Next"))
  (CallFunction|QuestCurrentTableStart _questtable))

(event EventQuestComplete
  (params (QuestName :type String))
  (Development|PrintString (Utilities|String|Append QuestName "__Complete") true true "(R=1.000000,G=0.006201,B=0.000000,A=1.000000)" 1e+01))

(event EventFinishedUpdateAchieve
  (params (AchieveNum :type String))
  (bind _asgm_solaseado (Utilities|Casting|CastToGM_Solaseado (Game|GetGameMode)))
  (Default|FindAchieve (Variables|/Game/Project/Widget/Menu/WB_MainMenu.WB_MainMenu_C|GetTest_PlayfabInterface (Variables|/Game/Project/World/GM_Solaseado.GM_Solaseado_C|GetWB_MainMenu _asgm_solaseado)) AchieveNum))

(fn ConstructionScript
  (Variables|Default|SetBP_SpringArm (Variables|Default|GetSpringArm))
  (Variables|Default|SetBP_ActorComponent_Playfab (Variables|Default|GetActorComponent_Playfab))
  (Class|SkinnedMeshComponent|SetMasterPoseComponent (Variables|Default|GetTop) (Variables|Default|GetBody) false)
  (Variables|/Script/Engine.SpringArmComponent|SetbUsePawnControlRotation (Variables|Default|GetSpringArm) false))

(fn GetCheckerCreateCharacter
  (return (Variables|/Script/Test_LidarSample.ActorComponent_Playfab|GetbCheckerCreateChracter (Variables|Default|GetActorComponent_Playfab))))

(fn GetUserCharacterName
  (return (Variables|/Script/Test_LidarSample.ActorComponent_Playfab|GetUserCharacterName (Variables|Default|GetActorComponent_Playfab))))

(fn ConnectPhotonAll
  (bind _asgm_solaseado (Utilities|Casting|CastToGM_Solaseado (Game|GetGameMode)))
  (Default|SpawnActorPhotonAll _asgm_solaseado))

(fn DefaultCameraSetting
  (bind _springarm (Variables|Default|GetSpringArm))
  (Variables|/Script/Engine.SpringArmComponent|SetTargetArmLength _springarm 3e+02)
  ;[1 1 1] body mesh에 상속되어서 z를 90 회전
  (Transformation|SetRelativeTransform _springarm (Math|Transform|MakeTransform "0,0.000000,180.000000" "-20.000000,90.000000, 0" "1,1,1") false false))