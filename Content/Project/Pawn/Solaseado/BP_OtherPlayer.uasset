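; BP_OtherPlayer is an actor Blueprint in the Solaseado pawn folder, named for other players' characters and built from modular body meshes.
; The construction script chains master pose components: Head and Hand follow Body, while Face, TempHandMesh and Hair follow Head.
; BeginPlay makes the Root and all its children visible.
; The overlap and Tick events are empty.
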(event EventBeginPlay
  (Rendering|SetVisibility (Variables|Default|GetRoot) true true))

(event Collision|EventActorBeginOverlap
  (params (OtherActor :type Actor%20Object%20Reference)))

(event EventTick
  (params (DeltaSeconds :type Float%20%28single-precision%29)))

(fn ConstructionScript
  (Class|SkinnedMeshComponent|SetMasterPoseComponent (Variables|Default|GetHead) (Variables|Default|GetBody) false)
  (Class|SkinnedMeshComponent|SetMasterPoseComponent (Variables|Default|GetFace) (Variables|Default|GetHead) false))