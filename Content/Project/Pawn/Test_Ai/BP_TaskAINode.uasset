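; Test behavior tree task that picks a navigable destination near the player when the controlled AI pawn is too far away.
; Beyond the distance threshold, it writes a random navmesh point around the player to a blackboard key and finishes with the query's result; otherwise it fails.
; The random query is pure and re-evaluates per use, so the debug-printed point can differ from the stored one.
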(event EventReceiveExecuteAI
  (params (OwnerController :type AI%20Controller%20Object%20Reference) (ControlledPawn :type Pawn%20Object%20Reference))
  (bind _returnvalue (Game|Player|GetPlayerPawn 0))
  (bind _returnvalue_2 (Transformation|GetActorLocation _returnvalue))
  (bind (_randomlocation _returnvalue_3) (Class|NavigationSystemV1|GetRandomPointinNavigableRadius _returnvalue_2 3e+02 0 0))
  (if (> (Math|Vector|Distance(Vector) _returnvalue_2 (Transformation|GetActorLocation ControlledPawn)) 5e+02)
    (Development|PrintString (Utilities|String|Append "// Test _Task Node DistValue :: " (Utilities|String|ToString(Vector) _randomlocation)))
    (AI|BehaviorTree|SetBlackboardValueasVector (Variables|Default|GetKey) _randomlocation)
    ;[1 1 1] 노드 종료 구문 없으면 다음 구조 실행 x
    (AI|BehaviorTree|FinishExecute _returnvalue_3)
    (else
      (AI|BehaviorTree|FinishExecute false))))