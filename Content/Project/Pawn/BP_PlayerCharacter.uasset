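; Player character pawn with a name tag, chat sent through the game mode's Photon client, and yaw-only camera rotation.
; A camera-mode toggle moves it to the "Start" PlayerStart, hides it and switches to UI-only input, then restores visibility.
; For mobile rendering, a switchable test overlap sphere culls nearby NPCs above a count limit, spawning one count-labelled dummy at the nearest's position until the crowd thins.
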(event OnComponentBeginOverlap(Test_Sphere)
  (params (OverlappedComponent :type Primitive%20Component%20Object%20Reference) (OtherActor :type Actor%20Object%20Reference) (OtherComp :type Primitive%20Component%20Object%20Reference) (OtherBodyIndex :type Integer) (bFromSweep :type Boolean) (SweepResult :type Hit%20Result%20Structure%20%28by%20ref%29))
  ;[1 0.1976 0.2175] // 모바일 최적화를 위한 캐릭터 랜더링 시스템
  (bind _astest_pawn_npc (Utilities|Casting|CastToTestPawn_npc OtherActor))
  (if (== (Variables|/Game/Project/Pawn/TestPawn_npc.TestPawn_npc_C|GetBox _astest_pawn_npc) OtherComp)
    (Utilities|Array|Add (Variables|Default|GetAs%20Test%20Pawn%20Npc) _astest_pawn_npc)
    (if (> (CallFunction|GetNPCLength) (Variables|Default|GetMaxCullingNPCCnt))
      (if (not (Variables|Default|GetbNPCCullingChecker))
        (Variables|Default|SetbNPCCullingChecker true)
        (for _array_element (Variables|Default|GetAs%20Test%20Pawn%20Npc)
          (Default|TestCharacterVisibleEffect _array_element false)
          (if (> (Variables|Default|GetTest_NPCtoPlayerDist) (Math|Vector|Distance(Vector) (Transformation|GetActorLocation (Game|Player|GetPlayerPawn 0)) (Transformation|GetActorLocation _array_element)))
            (Variables|Default|SetTest_NPCtoPlayerDist (Math|Vector|Distance(Vector) (Transformation|GetActorLocation (Game|Player|GetPlayerPawn 0)) (Transformation|GetActorLocation _array_element)))
            (Variables|Default|SetTest_DummyDistCheck _array_element)))
        (Utilities|IsValid (Variables|Default|GetTest_DummyDistCheck)
          (:Is%20Valid
            ;[1 0.1976 0.2175] Spawn AI Pawn
            (bind _returnvalue (Game|SpawnActorfromClass "/Game/Project/Pawn/TestPawn_npc_AI.TestPawn_npc_AI_C" (Transformation|GetActorTransform (Variables|Default|GetTest_DummyDistCheck)) "AlwaysSpawn" 0 true 0))
            (Variables|Default|SetNPCCullingPawn _returnvalue)
            (Development|PrintString "// Test _ Start Culling NPC ")
            (CallFunction|SetCullingNpcCnt)
            (Variables|Default|SetTest_NPCtoPlayerDist 9999.0))
          (:Is%20Not%20Valid
            (Development|PrintString "// Test _ Dummy Dist Checker :: NULL")))
        (else
          (CallFunction|SetCullingNpcCnt)
          (Default|TestCharacterVisibleEffect _astest_pawn_npc false))))))

(event OnComponentEndOverlap(Test_Sphere)
  (params (OverlappedComponent :type Primitive%20Component%20Object%20Reference) (OtherActor :type Actor%20Object%20Reference) (OtherComp :type Primitive%20Component%20Object%20Reference) (OtherBodyIndex :type Integer))
  (bind _npccullingpawn (Variables|Default|GetNPCCullingPawn))
  ;[1 0.1976 0.2175] // 모바일 최적화를 위한 캐릭터 랜더링 시스템
  (bind _astest_pawn_npc (Utilities|Casting|CastToTestPawn_npc OtherActor))
  (if (== (Variables|/Game/Project/Pawn/TestPawn_npc.TestPawn_npc_C|GetBox _astest_pawn_npc) OtherComp)
    (Utilities|Array|RemoveItem (Variables|Default|GetAs%20Test%20Pawn%20Npc) _astest_pawn_npc)
    (if (Variables|Default|GetbNPCCullingChecker)
      (if (<= (CallFunction|GetNPCLength) (Variables|Default|GetMaxCullingNPCCnt))
        (Variables|Default|SetbNPCCullingChecker false)
        (for _array_element (Variables|Default|GetAs%20Test%20Pawn%20Npc)
          (Default|TestCharacterVisibleEffect _array_element true))
        (Utilities|IsValid _npccullingpawn
          (:Is%20Valid
            (Actor|DestroyActor _npccullingpawn)))
        (else
          (Default|TestCharacterVisibleEffect _astest_pawn_npc true)
          (CallFunction|SetCullingNpcCnt))))))

(event Custom|WorldMessage
  (params (Message :type String) (type :type String))
  ;[1 1 1] 채팅 메세지
  (bind _asbp_gm (Utilities|Casting|CastToBP_GM (Game|GetGameMode)))
  (Class|ActorPhoton|SendTextMessage (Variables|/Game/Project/World/Test_LiDAR/BP_GM.BP_GM_C|GetPhotonClient _asbp_gm) Message type))

(event Custom|setCameraModeChange
  (bind _returnvalue (Game|GetPlayerController 0))
  (bind _relative_rotation (Variables|Default|GetRelative%20Rotation))
  (bind _mesh (Variables|Character|GetMesh))
  ;[1 1 1] 카메라 전환 기능 추가
  (Utilities|FlowControl|FlipFlop
    (:A
      (bind _returnvalue_2 (CallFunction|GetStartPoint))
      (Transformation|SetActorTransform (Math|Transform|MakeTransform (Math|Vector|MakeVector (.x _returnvalue_2) (.y _returnvalue_2) (.z (Transformation|GetActorLocation))) "0,-160.000000, 0" "1,1,1"))
      (Transformation|SetRelativeRotation (Variables|Default|GetSpringArmComp) (Math|Rotator|MakeRotator (.roll _relative_rotation) (.pitch _relative_rotation) 2e+02) false false)
      (Rendering|SetVisibility _mesh false false)
      (Input|SetInputModeUIOnly _returnvalue 0 "DoNotLock"))
    (:B
      (Rendering|SetVisibility _mesh true false)
      (Input|SetInputModeGameandUI _returnvalue 0 "DoNotLock" true))))

(event Custom|setCameraRotation_Pitch
  (params (Yaw :type Float%20%28single-precision%29))
  ;[1 0 0] 카메라 회전 :: 회전 차단 // z 축 회전만 사용
)

(event Custom|setCameraRotation_Yaw
  (params (Yaw :type Float%20%28single-precision%29))
  (bind _springarmcomp (Variables|Default|GetSpringArmComp))
  (bind _relativerotation (Variables|/Script/Engine.SceneComponent|GetRelativeRotation _springarmcomp))
  ;[1 1 1] 카메라 회전
  (Transformation|SetRelativeRotation _springarmcomp (Math|Rotator|MakeRotator (.roll _relativerotation) (.pitch _relativerotation) (+ (.yaw _relativerotation) (* Yaw 0.5))) false false))

(event Custom|Test_CullNPCRemove
  (bind _npccullingpawn (Variables|Default|GetNPCCullingPawn))
  (Variables|Default|SetbNPCCullingChecker false)
  (for _array_element (Variables|Default|GetAs%20Test%20Pawn%20Npc)
    (Default|TestCharacterVisibleEffect _array_element true))
  (Utilities|IsValid _npccullingpawn
    (:Is%20Valid
      (Actor|DestroyActor _npccullingpawn))))

(event EventSetPlayerNameTag
  (params (name :type String))
  ;[1 1 1] 네임 태그
  (bind _aswb_name_tag (Utilities|Casting|CastToWB_NameTag (UserInterface|GetUserWidgetObject (Variables|Default|GetNameTag))))
  (Class|WidgetNameTag|SetPlayerNametag _aswb_name_tag name)
  (Rendering|SetVisibility (Variables|Default|GetNameTag) true false))

(event EventBeginPlay
  (|CallParentFunction)
  (Rendering|Material|SetScalarParameterValueonMaterials (Variables|Default|GetHand) "Opacity" 1.0)
  (Variables|Default|SetRelative%20Rotation (Variables|/Script/Engine.SceneComponent|GetRelativeRotation (Variables|Default|GetSpringArmComp))))

(fn ConstructionScript
  (Class|SkinnedMeshComponent|SetMasterPoseComponent (Variables|Default|GetHand) (Variables|Character|GetMesh) false))

(fn GetStartPoint
  (bind _outactors (Actor|GetAllActorsOfClass "/Script/Engine.PlayerStart"))
  (for _array_element _outactors
    (for _array_element_2 (Variables|/Script/Engine.Actor|GetTags _array_element)
      (if (Utilities|Name|Equal(Name) _array_element_2 "Start")
        (return (Transformation|GetActorLocation _array_element))))))

(fn GetNPCLength
  (return (Utilities|Array|Length (Variables|Default|GetAs%20Test%20Pawn%20Npc))))

(fn SetCullingNpcCnt
  (bind _npccullingpawn (Variables|Default|GetNPCCullingPawn))
  (Utilities|IsValid _npccullingpawn
    (:Is%20Valid
      (Default|TestNPCMarkerNumber _npccullingpawn (Utilities|String|ToString(Integer) (CallFunction|GetNPCLength)))
      (Default|SetNameTagBP _npccullingpawn "Test_Culling"))
    (:Is%20Not%20Valid
      (Development|PrintString "// Test _ Error Culling NPC :: NULL"))))

(fn SetMaxWalkSpeed
  (params (Max%20Walk%20Speed :type Float%20%28single-precision%29))
  (Variables|/Script/Engine.CharacterMovementComponent|SetMaxWalkSpeed (Variables|Character|GetCharacterMovement) Max%20Walk%20Speed))

(fn SetCullingSystem
  (params (bON :type Boolean))
  (bind _test_sphere (Variables|Default|GetTest_Sphere))
  (if bON
    (Collision|SetCollisionEnabled _test_sphere "QueryOnly")
    (else
      (Collision|SetCollisionEnabled _test_sphere "NoCollision")
      ;[1 1 1] 기존 컬링 처리 제거
      (CallFunction|TestCullNPCRemove))))