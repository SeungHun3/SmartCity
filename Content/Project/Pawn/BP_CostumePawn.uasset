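; Costume pawn for character customization that shows a modular skeletal character and steers the login pawn's camera between tabs.
; Construction slaves head and hand meshes to Body, and face and hair to Head, with custom depth on the latter two.
; Scene changes send the camera to the full-shot point or a selected part's position.
; BP Select Position finds that point by matching a data-table name to a mesh's "Scene"-suffixed child.
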(event EventBeginPlay
  (bind _asbp_login_pawn (Utilities|Casting|CastToBP_LoginPawn (Game|Player|GetPlayerPawn 0)))
  (Variables|Default|SetAs%20BP%20Login%20Pawn _asbp_login_pawn))

(event Collision|EventActorBeginOverlap
  (params (OtherActor :type Actor%20Object%20Reference)))

(event EventTick
  (params (DeltaSeconds :type Float%20%28single-precision%29)))

(fn ConstructionScript
  (Class|SkinnedMeshComponent|SetMasterPoseComponent (Variables|Default|GetHand) (Variables|Default|GetBody) false)
  (Class|SkinnedMeshComponent|SetMasterPoseComponent (Variables|Default|GetFace) (Variables|Default|GetHead) false)
  (Rendering|SetRenderCustomDepth (Variables|Default|GetFace) true))

(fn BPSelectPosition
  (params (ClassName :type Integer))
  (bind _asgame_instance_solaseado (Utilities|Casting|CastToGameInstance_Solaseado (Game|GetGameInstance)))
  (bind _returnvalue (Utilities|GetDataTableRow (Utilities|Array|Get(acopy) (Class|GameInstanceSolaseado|GetDataTables _asgame_instance_solaseado) ClassName) "1")
    (:then
      (bind _output_get (Variables|Default|SetDataTable _returnvalue))
      (for _array_element (Actor|GetComponentsByClass "/Script/Engine.SkeletalMeshComponent")
        (if (Utilities|Enum|Equal(Enum) (Utilities|GetObjectName _array_element) (.classname _output_get))
          (for _array_element_2 (Components|GetChildrenComponents _array_element false)
            (if (Utilities|Enum|Equal(Enum) (Utilities|GetObjectName _array_element_2) (Utilities|String|Append (Utilities|GetObjectName _array_element) "Scene"))
              (return true (Transformation|GetWorldLocation _array_element_2))))))
      (return false "0, 0, 0"))))

(fn BindInit
  (params (WB_Customizing_Tab :type Widget%20Customizing%20Tab%20Object%20Reference))
  ;[1 1 1] 아직 내용없음
  (bind _returnvalue (|CallParentFunction WB_Customizing_Tab))
  (EventDispatchers|BindEventtoChangeSlotDelegate WB_Customizing_Tab (EventDispatchers|CreateEvent :!event ChangeScene))
  (return _returnvalue))

(fn ChangeScene
  (params (TabNumber :type Integer))
  ;[1 1 1] 아직 내용없음
  (|CallParentFunction TabNumber)
  (bind _asgm_solaseado (Utilities|Casting|CastToGM_Solaseado (Game|GetGameMode)))
  (if (Variables|/Script/Test_LidarSample.Widget_Customizing|GetIsFullShot (Variables|/Script/Test_LidarSample.PlayerState_Solaseado|GetWidget_Customizing (Class|GameModeBaseSolaseado|GetPlayerStateSolaseado _asgm_solaseado)))
    ;[1 1 1] 전체화면
    (Default|CameraTimeLine (Variables|Default|GetAs%20BP%20Login%20Pawn) (Transformation|GetWorldLocation (Variables|Default|GetFullScene)))
    (return)
    (else
      (bind (_isfind _location) (CallFunction|SelectPosition TabNumber))
      (if _isfind
        (Default|CameraTimeLine (Variables|Default|GetAs%20BP%20Login%20Pawn) _location)
        (return)))))