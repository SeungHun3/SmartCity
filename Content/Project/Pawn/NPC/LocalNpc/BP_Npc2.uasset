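; BP_Npc2 is a local NPC that offers dialogue and quest interaction when the player comes near.
; On BeginPlay it shows its NPC mark and sets its displayed name.
; When a BP_LoginPawn component tagged "Player" enters its Box, it enables the GM_Solaseado dialogue button, starts its quest there and calls QuestableNpc.
; Leaving the Box unbinds the dialogue button to avoid clashes with other NPCs.
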(event OnComponentBeginOverlap(Box)
  (params (OverlappedComponent :type Primitive%20Component%20Object%20Reference) (OtherActor :type Actor%20Object%20Reference) (OtherComp :type Primitive%20Component%20Object%20Reference) (OtherBodyIndex :type Integer) (bFromSweep :type Boolean) (SweepResult :type Hit%20Result%20Structure%20%28by%20ref%29))
  (bind _questname (Variables|Default|GetQuestName))
  (Utilities|Casting|CastToBP_LoginPawn OtherActor)
  (if (Components|ComponentHasTag OtherComp "Player")
    (bind _asgm_solaseado (Utilities|Casting|CastToGM_Solaseado (Game|GetGameMode)))
    (Default|SetNpcDialogueButton _asgm_solaseado true "Visible" (Variables|Default|GetNpcName))
    (Default|NpcQuestStart _asgm_solaseado _questname self)
    (CallFunction|QuestableNpc _questname)))

(event OnComponentEndOverlap(Box)
  (params (OverlappedComponent :type Primitive%20Component%20Object%20Reference) (OtherActor :type Actor%20Object%20Reference) (OtherComp :type Primitive%20Component%20Object%20Reference) (OtherBodyIndex :type Integer))
  (Utilities|Casting|CastToBP_LoginPawn OtherActor)
  (if (Components|ComponentHasTag OtherComp "Player")
    (bind _asgm_solaseado (Utilities|Casting|CastToGM_Solaseado (Game|GetGameMode)))
    (Default|DialogueButtonUnbinding _asgm_solaseado)))

(event EventBeginPlay
  (|CallParentFunction)
  (CallFunction|SetNpcMarkVisibility true)
  (CallFunction|SetNpcName (Utilities|Text|ToText(Name) (Variables|Default|GetNpcName))))

(event Collision|EventActorBeginOverlap
  (params (OtherActor :type Actor%20Object%20Reference)))

(event EventTick
  (params (DeltaSeconds :type Float%20%28single-precision%29))
  (|CallParentFunction DeltaSeconds) ; 지금 이 노드는 비활성 상태입니다. \n핀을 끌어서 다른 노드를 연결하면 활성화됩니다.
)

(fn ConstructionScript
  (|CallParentFunction))