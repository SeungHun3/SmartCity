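; BP_SolaseadoPhoton is the Solaseado game's Photon client actor, relaying networking events from its parent class to the rest of the game.
; On BeginPlay it registers itself as BPPhotonCloud on the PC_Solaseado player controller.
; View count changes and player add, remove and reset events are re-broadcast through event dispatchers, while player data initialization defers to the parent.
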(event EventInitPlayerData
  (|CallParentFunction))

(event EventBlueprintAddPlayer
  (params (PlayerNr :type Integer) (name :type String))
  ;[1 1 1] Test Widget Checker
  (Default|CallDispatcherAddPlayer PlayerNr name))

(event EventBeginPlay
  (bind _aspc_solaseado (Utilities|Casting|CastToPC_Solaseado (Game|GetPlayerController 0)))
  (Variables|/Game/Project/World/PC_Solaseado.PC_Solaseado_C|SetBP_Photon_Cloud _aspc_solaseado self))

(event EventChangeViewCount
  (params (Channel_Count :type Map%20of%20Integers%20to%20Integers) (PlayerNames :type Array%20of%20Strings))
  (Default|CallCallRoomSlot Channel_Count))

(event EventBlueprintRemovePlayer
  (params (PlayerNr :type Integer))
  ;[1 1 1] Test Widget Checker
  (Default|CallDispatcherRemovePlayer PlayerNr))

(event EventBlueprintResetPlayer
  (Default|CallDispatcherResetPlayer))

(fn ConstructionScript)