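; BP_OXPanel is the O/X quiz panel actor that lights up its O and X meshes while a question is presented and when an answer is shown.
; A looping one-second timer flip-flops the Emissive material parameter, blinking O and X alternately alongside a selection sound on the Audio component.
; Effect_O and Effect_X light one side and play a shared sound; ActiveSound toggles the audio, stops the timer and clears both glows.
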(event Custom|Emissive_OX
  (Utilities|FlowControl|FlipFlop
    (:A
      (Variables|Default|SetParameter%20Value 0.0))
    (:B
      (Variables|Default|SetParameter%20Value 1e+02)))
  (Rendering|Material|SetScalarParameterValueonMaterials (Variables|Default|GetS_OX_line_S_OX_O) "Emissive" (Variables|Default|GetParameter%20Value))
  (Rendering|Material|SetScalarParameterValueonMaterials (Variables|Default|GetS_OX_line_S_OX_X) "Emissive" (- 1e+02 (Variables|Default|GetParameter%20Value))))

(event Custom|QuizSelectSoundAndEffect
  (bind _audio (Variables|Default|GetAudio))
  ;[1 1 1] 사운드 플레이
  (Audio|Components|Audio|SetSound _audio "/Game/Project/Sound/M1_SFX_02.M1_SFX_02")
  (Components|Activation|SetActive _audio true true)
  (CallFunction|QuizSelectEffect))

(event Custom|ActiveSound
  (params (bActive :type Boolean))
  ;[1 1 1] 사운드 활성화 여부
  (Components|Activation|SetActive (Variables|Default|GetAudio) bActive true)
  (Utilities|Time|ClearandInvalidateTimerbyHandle (Variables|Default|GetEffectHandle))
  (Rendering|Material|SetScalarParameterValueonMaterials (Variables|Default|GetS_OX_line_S_OX_O) "Emissive" 0.0)
  (Rendering|Material|SetScalarParameterValueonMaterials (Variables|Default|GetS_OX_line_S_OX_X) "Emissive" 0.0))

(event Custom|QuizSelectEffect
  ;[1 1 1] 문제 출력 이펙트
  (bind _returnvalue (Utilities|Time|SetTimerbyEvent (delegate Custom|Emissive_OX) 1.0 true))
  (Variables|Default|SetEffectHandle _returnvalue))

(event Custom|Effect_X
  ;[1 1 1] OX 마커 정답 이펙
  (Rendering|Material|SetScalarParameterValueonMaterials (Variables|Default|GetS_OX_line_S_OX_X) "Emissive" 1e+02)
  ;[1 1 1] 조명이 정답쪽에 멈출때
  (Audio|PlaySound2D "/Game/Project/Sound/M1_SFX_05.M1_SFX_05" 1.0 1.0 0.0 0 0))

(event Custom|Effect_O
  ;[1 1 1] OX 마커 정답 이펙
  (Rendering|Material|SetScalarParameterValueonMaterials (Variables|Default|GetS_OX_line_S_OX_O) "Emissive" 1e+02)
  ;[1 1 1] 조명이 정답쪽에 멈출때
  (Audio|PlaySound2D "/Game/Project/Sound/M1_SFX_05.M1_SFX_05" 1.0 1.0 0.0 0 0))

(fn ConstructionScript)