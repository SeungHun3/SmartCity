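; BP_AR is an AR controller actor that toggles an AR session together with device location services.
; Init sets up location services, and PressBTN starts or stops them through the CheckAR guard on init and running state.
; On success, SetStart hides or restores the BP_Sky_Sphere and starts or stops the AR session.
; While running, Tick stores the last known location and prints its fields for debugging.
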(event EventTick
  (params (DeltaSeconds :type Float%20%28single-precision%29))
  (if (Variables|Default|GetIs_Start)
    (bind _returnvalue (Class|LocationServices|GetLastKnownLocation))
    (bind _output_get (Variables|Default|SetLocation _returnvalue))
    (Development|PrintString (Utilities|String|Append "Timestamp__" (Utilities|String|ToString(Float) (.Timestamp (Utilities|Struct|BreakLocationServicesData _output_get))) "__Longitude__" (Utilities|String|ToString(Float) (.Longitude (Utilities|Struct|BreakLocationServicesData _output_get))) "__Latitude__" (Utilities|String|ToString(Float) (.Latitude (Utilities|Struct|BreakLocationServicesData _output_get))) "__Horizon__" (Utilities|String|ToString(Float) (.HorizontalAccuracy (Utilities|Struct|BreakLocationServicesData _output_get))) "__Vertical__" (Utilities|String|ToString(Float) (.VerticalAccuracy (Utilities|Struct|BreakLocationServicesData _output_get))) "__Altitude__" (Utilities|String|ToString(Float) (.Altitude (Utilities|Struct|BreakLocationServicesData _output_get)))))))

(fn ConstructionScript)

(fn Init
  (bind _returnvalue (Class|LocationServices|AreLocationServicesEnabled))
  (if _returnvalue
    (bind _returnvalue_2 (Class|LocationServices|InitLocationServices "LA_ThreeKilometers" 0.02 1.0))
    (Variables|Default|SetIs_Init _returnvalue_2)))

(fn SetStart
  (params (Is_Start :type Boolean))
  (bind _output_get (Variables|Default|SetIs_Start Is_Start))
  (if _output_get
    (bind _returnvalue (Actor|GetActorOfClass "/Engine/EngineSky/BP_Sky_Sphere.BP_Sky_Sphere_C"))
    (Utilities|IsValid _returnvalue
      (:Is%20Valid
        (Rendering|SetVisibility (Variables|/Engine/EngineSky/BP_Sky_Sphere.BP_Sky_Sphere_C|GetBase _returnvalue) false true)
        (Class|ARBlueprintLibrary|StartARSession "/Game/Project/World/AR_DataAsset.AR_DataAsset")))
    (else
      (bind _returnvalue_2 (Actor|GetActorOfClass "/Engine/EngineSky/BP_Sky_Sphere.BP_Sky_Sphere_C"))
      (Utilities|IsValid _returnvalue_2
        (:Is%20Valid
          (Rendering|SetVisibility (Variables|/Engine/EngineSky/BP_Sky_Sphere.BP_Sky_Sphere_C|GetBase _returnvalue_2) true true)
          (Class|ARBlueprintLibrary|StopARSession))))))

(fn PressBTN
  (params (IsStart :type Boolean))
  (if IsStart
    (Utilities|CheckAR
      (:CanStart
        (bind _returnvalue (Class|LocationServices|StartLocationServices))
        (if _returnvalue
          (CallFunction|SetStart _returnvalue))))
    (else
      (Utilities|CheckAR
        (:CanStop
          (bind _returnvalue_2 (Class|LocationServices|StopLocationServices))
          (if _returnvalue_2
            (CallFunction|SetStart (not _returnvalue_2))))))))