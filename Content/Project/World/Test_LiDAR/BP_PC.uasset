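; Player controller for the LiDAR test world that turns camera, zoom, sprint, cursor and chat inputs into actions on the cached BP_PlayerCharacter.
; Axis inputs rotate the camera, while mouse wheel and two-finger pinch adjust clamped spring arm length; the wheel also repositions the message box and name tag.
; Shift temporarily sets walk speed, Ctrl toggles the cursor and Enter focuses the main widget.
; An auto-move goal event starts looping movement on the first BP_Spline found.
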(event EventAutoMoveGoalEvent
  ;[1 1 1] 자동이동 탐색 종료 >> 순환 이동
  (bind _outactors (Actor|GetAllActorsOfClass "/Game/Project/Actor/BP_Spline.BP_Spline_C"))
  (Utilities|IsValid (Utilities|Array|Get(acopy) _outactors)
    (:Is%20Valid
      (Default|MoveSplineTimerEvent (Utilities|Array|Get(acopy) _outactors)))))

(event EventBeginPlay
  (bind _asbp_player_character (Utilities|Casting|CastToBP_PlayerCharacter (Game|Player|GetPlayerPawn 0)))
  (Variables|Default|SetAs%20BP%20Player%20Character _asbp_player_character))

(event Input|AxisEvents|InputAxisUp
  (params (AxisValue :type Float%20%28single-precision%29))
  (bind _as_bp_player_character (Variables|Default|GetAs%20BP%20Player%20Character))
  ;[1 1 1] 카메라 회전
  (if (!= AxisValue 0.0)
    (Utilities|IsValid _as_bp_player_character
      (:Is%20Valid
        (Default|SetCameraRotationYaw _as_bp_player_character AxisValue)))))

(event Input|AxisEvents|InputAxisMouseX
  (params (AxisValue :type Float%20%28single-precision%29))
  (bind _as_bp_player_character (Variables|Default|GetAs%20BP%20Player%20Character))
  (if (!= AxisValue 0.0)
    (Utilities|IsValid _as_bp_player_character
      (:Is%20Valid
        (Default|SetCameraRotationYaw _as_bp_player_character AxisValue)))))

(event Input|AxisEvents|InputAxisMouseWheel
  (params (AxisValue :type Float%20%28single-precision%29))
  (bind _as_bp_player_character (Variables|Default|GetAs%20BP%20Player%20Character))
  (bind _messagebox (Variables|/Script/Test_LidarSample.Character_Player|GetMessageBox _as_bp_player_character))
  (bind _nametag (Variables|/Game/Project/Pawn/BP_PlayerCharacter.BP_PlayerCharacter_C|GetNameTag _as_bp_player_character))
  (bind _springarmcomp (Variables|/Script/Test_LidarSample.Character_Player|GetSpringArmComp _as_bp_player_character))
  (bind _relativelocation (Variables|/Script/Engine.SceneComponent|GetRelativeLocation _messagebox))
  (bind _relativelocation_2 (Variables|/Script/Engine.SceneComponent|GetRelativeLocation _nametag))
  ;[1 1 1] 마우스 휠 // 카메라 줌인 아웃
  (if (!= AxisValue 0.0)
    (bind _output_get (Variables|/Script/Engine.SpringArmComponent|SetTargetArmLength _springarmcomp (Math|Float|Clamp(Float) (+ (Variables|/Script/Engine.SpringArmComponent|GetTargetArmLength _springarmcomp) (* AxisValue -1e+01)) 5e+01 2.5e+02)))
    (Transformation|SetRelativeLocation _messagebox (Math|Vector|MakeVector _output_get (.y _relativelocation) (.z _relativelocation)) false false)
    (Transformation|SetRelativeLocation _nametag (Math|Vector|MakeVector _output_get (.y _relativelocation_2) (.z _relativelocation_2)) false false)))

(event Input|AxisEvents|InputAxisMouseY
  (params (AxisValue :type Float%20%28single-precision%29))
  (bind _as_bp_player_character (Variables|Default|GetAs%20BP%20Player%20Character))
  (if (!= AxisValue 0.0)
    (Utilities|IsValid _as_bp_player_character
      (:Is%20Valid
        (Default|SetCameraRotationPitch _as_bp_player_character AxisValue)))))

(event Input|KeyboardEvents|Enter
  (params (Key :type Key%20Structure))
  ;[1 1 1] 채팅 입력
  (:Pressed
    (bind _aswb_main (Utilities|Casting|CastToWB_Main (Variables|/Script/Test_LidarSample.Character_Player|GetMainWidget (Variables|Default|GetAs%20BP%20Player%20Character))))
    (Default|SetKeyvoardFocus _aswb_main)))

(event Input|KeyboardEvents|LeftShift
  (params (Key :type Key%20Structure))
  (bind _as_bp_player_character (Variables|Default|GetAs%20BP%20Player%20Character))
  (bind _charactermovement (Variables|/Script/Engine.Character|GetCharacterMovement _as_bp_player_character))
  ;[1 1 1] move Controller Key
  (:Pressed
    (Variables|Default|SetCurrentSpeed (Variables|/Script/Engine.CharacterMovementComponent|GetMaxWalkSpeed _charactermovement))
    (Variables|/Script/Engine.CharacterMovementComponent|SetMaxWalkSpeed _charactermovement 3.5e+02))
  (:Released
    (Variables|/Script/Engine.CharacterMovementComponent|SetMaxWalkSpeed _charactermovement (Variables|Default|GetCurrentSpeed))))

(event Input|KeyboardEvents|LeftCtrl
  (params (Key :type Key%20Structure))
  (:Pressed
    (Development|PrintString "Hello")
    (Utilities|FlowControl|FlipFlop
      (:A
        (Variables|Default|SetbShowMouseCursor false))
      (:B
        (Variables|Default|SetbShowMouseCursor true)))))

(event Input|TouchEvents|InputTouch
  (params (Location :type Vector) (FingerIndex :type ETouchIndex%20Enum))
  (bind _as_bp_player_character (Variables|Default|GetAs%20BP%20Player%20Character))
  (bind _springarmcomp (Variables|/Script/Test_LidarSample.Character_Player|GetSpringArmComp _as_bp_player_character))
  (:Pressed
    (switch Utilities|FlowControl|Switch|SwitchonETouchIndex FingerIndex
      (:Touch1
        (Variables|Default|SetbTouch1 true))
      (:Touch2
        (Variables|Default|SetbTouch2 true)
        (Variables|Default|SetTouchDist (Math|Vector|Distance(Vector) (Variables|Default|GetTouch1Loc) (Variables|Default|GetTouch2Loc))))))
  (:Released
    (switch Utilities|FlowControl|Switch|SwitchonETouchIndex FingerIndex
      (:Touch1
        (Variables|Default|SetbTouch1 false))
      (:Touch2
        (Variables|Default|SetbTouch2 false)
        (Variables|Default|SetTouchDist 0.0))))
  (:Moved
    (if (and (Variables|Default|GetbTouch1) (Variables|Default|GetbTouch2))
      (switch Utilities|FlowControl|Switch|SwitchonETouchIndex FingerIndex
        (:Touch1
          (Variables|Default|SetTouch1Loc Location))
        (:Touch2
          (Variables|Default|SetTouch2Loc Location)))
      (bind _output_get (Variables|/Script/Engine.SpringArmComponent|SetTargetArmLength _springarmcomp (Math|Float|Clamp(Float) (+ (Variables|/Script/Engine.SpringArmComponent|GetTargetArmLength _springarmcomp) (/ (- (Variables|Default|GetTouchDist) (Math|Vector|Distance(Vector) (Variables|Default|GetTouch1Loc) (Variables|Default|GetTouch2Loc))) 2.0)) 5e+01 2.5e+02)))
      (Development|PrintString (Utilities|String|ToString(Float) _output_get)))))

(fn ConstructionScript)