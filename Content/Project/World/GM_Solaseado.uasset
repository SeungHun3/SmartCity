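; Solaseado game mode that starts the game in the Intro level and manages UI screens, level arrival and Photon connections.
; When a streamed level finishes, it moves the pawn to the PlayerStart tagged with that level's name, then shows intro, customizing or main menu UI.
; The Login level temporarily serves as the customizing scene; login UI follows the loading widget.
; Separate events spawn Photon chat, voice and cloud clients using the login pawn's character name.
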(event Custom|SpawnActor_PhotonVoice
  ;[1 1 1] // Photon Voice Client
  (Development|PrintString "// Connect Voice ")
  (bind _returnvalue (Game|SpawnActorfromClass "/Game/Project/Actor/PhotonVoice/PhotonVoiceClient.PhotonVoiceClient_C" (Math|Transform|MakeTransform "0, 0, 0") "AlwaysSpawn" 0 0))
  (bind _output_get (Variables|Default|SetPhotonVoiceClient _returnvalue))
  (bind _asbp_login_pawn (Utilities|Casting|CastToBP_LoginPawn (Game|Player|GetPlayerPawn 0)))
  (Utilities|IsValid (Variables|/Game/Project/Pawn/Solaseado/BP_LoginPawn.BP_LoginPawn_C|GetActorComponent_Playfab _asbp_login_pawn)
    (:Is%20Valid
      (Class|ActorPhotonVoice|Connect _output_get (Variables|/Script/Test_LidarSample.ActorComponent_Playfab|GetUserCharacterName (Variables|/Game/Project/Pawn/Solaseado/BP_LoginPawn.BP_LoginPawn_C|GetActorComponent_Playfab _asbp_login_pawn))))))

(event Custom|OnEndLoading
  ;[1 1 1] Loading Widget 추가 / SJW
  (CallFunction|SolaseadoLogin))

(event Custom|UIMainMenu
  ;[1 1 1] MainMenuWidget 생성
  (Development|PrintString "// Widget :: UIMainMenu")
  (Viewport|RemoveAllWidgets)
  (bind _returnvalue (UserInterface|CreateWidget "/Game/Project/Widget/Chating/WB_MainMenu.WB_MainMenu_C"))
  (bind _output_get (Variables|Default|SetWB_MainMenu _returnvalue))
  (UserInterface|Viewport|AddtoViewport _output_get 0))

(event Custom|WidgetCreate_Intro
  (Development|PrintString "// Widget :: Intro")
  ;[1 1 1] Intro Widget 추가
  (Viewport|RemoveAllWidgets)
  (bind _returnvalue (UserInterface|CreateWidget "/Game/Project/Widget/WB_Intro.WB_Intro_C"))
  (bind _output_get (Variables|Default|SetWidget_Intro _returnvalue))
  (UserInterface|Viewport|AddtoViewport _output_get 0))

(event Custom|SpawnActor_PhotonChat
  ;[1 1 1] Photon Chat
  (bind _returnvalue (Game|SpawnActorfromClass "/Game/Project/Actor/PhotonChat/PhotonChatClient.PhotonChatClient_C" (Math|Transform|MakeTransform "0, 0, 0") "AlwaysSpawn" 0 0))
  (bind _output_get (Variables|Default|SetPhotonChatClient _returnvalue))
  (bind _asbp_login_pawn (Utilities|Casting|CastToBP_LoginPawn (Game|Player|GetPlayerPawn 0)))
  (Development|PrintString (Utilities|String|Append "// Check _ PlayerName :: " (Default|GetUserCharacterName _asbp_login_pawn)))
  (Class|ActorPhotonChat|ConnectChat _output_get (Default|GetUserCharacterName _asbp_login_pawn)))

(event Custom|StreamLevelFinish_Event_0
  (params (level :type String))
  ;[0 0.6099 1] // Intro  시작 & 레벨 이동 델리게이트 이벤트 바인딩 / StreamLevelFinish
  ;;[1 1 1] 레벨 이동에 따른 설정 추가 하기
  (CallFunction|SetLevelLoadFinishedEvent level))

(event Custom|Solaseado_Login
  ;[1 1 1] // Login Widget / Intro 이후 로그인 적용
  (bind _returnvalue (UserInterface|CreateWidget "/Game/Project/Widget/WB_SolaseadoLogin.WB_SolaseadoLogin_C"))
  (bind _output_get (Variables|Default|SetWidget_SolaseadoLogin _returnvalue))
  (UserInterface|Viewport|AddtoViewport _output_get 0))

(event Custom|SpawnActor_PhotonCloud
  ;[1 1 1] PhotonCloud
  (bind _returnvalue (Game|SpawnActorfromClass "/Game/Project/Actor/PhotonClient/BP_SolaseadoPhoton.BP_SolaseadoPhoton_C" (Math|Transform|MakeTransform "0, 0, 0") "AlwaysSpawn" 0 0))
  (bind _output_get (Variables|Default|SetPhotonCloud _returnvalue))
  (bind _asbp_login_pawn (Utilities|Casting|CastToBP_LoginPawn (Game|Player|GetPlayerPawn 0)))
  (Class|ActorSolaseadoPhoton|ConnectLogin _output_get (Default|GetUserCharacterName _asbp_login_pawn))
  (Development|PrintString "// Photon_Connect"))

(event Custom|WidgetCreate_Loading
  ;[1 1 1] Loading Widget 추가 / SJW
  (Development|PrintString "// Widget :: Loading")
  (Viewport|RemoveAllWidgets)
  (bind _returnvalue (UserInterface|CreateWidget "/Game/Project/Widget/intro/WB_Loading.WB_Loading_C"))
  (bind _output_get (Variables|Default|SetWB_Loading _returnvalue))
  (UserInterface|Viewport|AddtoViewport _output_get 0)
  (EventDispatchers|BindEventtoOnEndLoading _output_get (delegate Custom|OnEndLoading)))

(event Custom|UICustomizing
  ;[1 1 1] CustomizingUI
  (Development|PrintString "// Widget :: UICustomizing")
  (Viewport|RemoveAllWidgets)
  (bind _returnvalue (UserInterface|CreateWidget "/Game/Project/Widget/Customizing/WB_Customizing.WB_Customizing_C"))
  (bind _output_get (Variables|Default|SetWidget_Customizing _returnvalue))
  (UserInterface|Viewport|AddtoViewport _output_get 0))

(event Custom|Create_Nickname
  ;[1 1 1] NicknameWidget 생성
  (bind _returnvalue (UserInterface|CreateWidget "/Game/Project/Widget/Customizing/WB_CreateNickname.WB_CreateNickname_C"))
  (bind _output_get (Variables|Default|SetWB_Create_Nickname _returnvalue))
  (UserInterface|Viewport|AddtoViewport _output_get 0))

(event EventBeginPlay
  ;[0 0.6099 1] // Intro  시작 & 레벨 이동 델리게이트 이벤트 바인딩 / StreamLevelFinish
  (EventDispatchers|AssignStreamLevelFinish (delegate Custom|StreamLevelFinish_Event_0))
  ;;[1 1 1] Defualt Level Load // Intro
  (Class|GameModeBaseSolaseado|FastMoveLevel "Intro"))

(fn ConstructionScript)

(fn SetStartPointMoveLocation
  (params (Level :type String))
  ;[1 1 1] Level > Player Start tag 비교
  (bind _outactors (Actor|GetAllActorsOfClass "/Script/Engine.PlayerStart"))
  (for _array_element _outactors
    (if (Utilities|Name|Equal(Name) (Variables|/Script/Engine.PlayerStart|GetPlayerStartTag _array_element) (Utilities|String|StringToName Level))
      ;[1 0.2552 0.2552] Pawn위치 Transform으로 변경
      (Transformation|SetActorTransform (Game|Player|GetPlayerPawn 0) (Math|Transform|MakeTransform (.location (Transformation|GetActorTransform _array_element)) "0,180.000000, 0" "1,1,1"))
      (Development|PrintString (Utilities|String|Append "// Player Pawn Set Location :: " (Utilities|String|ToString(Name) (Variables|/Script/Engine.PlayerStart|GetPlayerStartTag _array_element))))
      (return))))

(fn SetLevelLoadFinishedEvent
  (params (Level :type String))
  (CallFunction|SetStartPointMoveLocation Level)
  (Utilities|Casting|CastToGM_Solaseado (Game|GetGameMode))
  (switch string Level
    (:Intro
      (Development|PrintString "// Check move Level :: Intro")
      (CallFunction|WidgetCreateIntro))
    (:Login
      ;[1 0.1976 0.2175] Login Level 을 임시 커스터마이징 씬으로 활용.
      (CallFunction|UICustomizing))
    (:SimPoly1
      (Development|PrintString "// Check move Level :: inGame ")
      (CallFunction|UIMainMenu))))