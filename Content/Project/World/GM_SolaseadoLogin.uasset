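; Game mode for the Solaseado login flow that switches between the login, character creation and main UI screens.
; On BeginPlay it shows the login widget with UI-only input and a visible cursor.
; Custom events clear all widgets to show character creation or the temporary in-game main widget.
; Another event spawns a Photon chat client and connects it using the character name from BP_LoginPawn.
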(event Custom|WidgetCreate_TitleUserID
  ;[1 1 1] Create Character
  (Viewport|RemoveAllWidgets)
  (bind _returnvalue (UserInterface|CreateWidget "/Game/Project/Widget/WB_CreateCharacter.WB_CreateCharacter_C"))
  (bind _output_get (Variables|Default|SetWidget_CreateChracter _returnvalue))
  (UserInterface|Viewport|AddtoViewport _output_get 0))

(event Custom|WidgetCreate_JoinGame
  ;[1 0.1976 0.2175] 임시 메인 위젯 / 채팅 기능 추가
  ;;[1 1 1] Ingame Widget 추가
  (Viewport|RemoveAllWidgets)
  (bind _returnvalue (UserInterface|CreateWidget "/Game/Project/Widget/WB_SolaseadoMain.WB_SolaseadoMain_C"))
  (bind _output_get (Variables|Default|SetWidget_SolaseadoMain _returnvalue))
  (UserInterface|Viewport|AddtoViewport _output_get 0))

(event Custom|SpawnActor_PhotonChat
  (bind _returnvalue (Game|SpawnActorfromClass "/Game/Project/Actor/PhotonChat/PhotonChatClient.PhotonChatClient_C" (Math|Transform|MakeTransform "0, 0, 0") "AlwaysSpawn" 0 0))
  (bind _output_get (Variables|Default|SetPhotonChatClient _returnvalue))
  (bind _asbp_login_pawn (Utilities|Casting|CastToBP_LoginPawn (Game|Player|GetPlayerPawn 0)))
  (Development|PrintString (Utilities|String|Append "// Check _ PlayerName :: " (Default|GetUserCharacterName _asbp_login_pawn)))
  (Class|ActorPhotonChat|ConnectChat _output_get (Default|GetUserCharacterName _asbp_login_pawn)))

(event EventBeginPlay
  (bind _returnvalue (Game|GetPlayerController 0))
  ;[1 1 1] Login Widget
  (bind _returnvalue_2 (UserInterface|CreateWidget "/Game/Project/Widget/WB_SolaseadoLogin.WB_SolaseadoLogin_C"))
  (bind _output_get (Variables|Default|SetWidget_SolaseadoLogin _returnvalue_2))
  (UserInterface|Viewport|AddtoViewport _output_get 0)
  (Input|SetInputModeUIOnly _returnvalue 0 "DoNotLock")
  (Variables|/Script/Engine.PlayerController|SetbShowMouseCursor _returnvalue true))

(fn ConstructionScript)