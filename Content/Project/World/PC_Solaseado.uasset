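; Player controller for Solaseado that handles movement, touch camera and test hotkeys, syncing movement through Photon.
; Axis and one-finger yaw input go to the GameMode's PhotonCloud only on change, while local movement paths sit disconnected.
; Tick moves BP_LoginPawn from its FForward, FRight and FRotationX values, turning via control rotation.
; Touch drags apply pitch locally, and two-finger gestures adjust clamped spring-arm length, reporting it to the menu widget.
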(event Custom|moveForwardKES
  (params (InputValue :type Float%20%28single-precision%29))
  (bind _as_bp_login_pawn (Variables|Default|GetAs%20BP%20Login%20Pawn))
  ;[1 1 1] 이동 입력축
  (Utilities|IsValid _as_bp_login_pawn
    (:Is%20Valid
      (Utilities|FlowControl|Sequence
        (:then_0
          (if (!= InputValue 0.0)
            (if (> InputValue 0.0)
              (Variables|Default|SetInputForwardValue "Forward")
              (else
                (Variables|Default|SetInputForwardValue "Back")))
            (else
              (Variables|Default|SetInputForwardValue "ForwardStop"))))
        (:then_1
          (if (Utilities|Enum|NotEqual(Enum) (Variables|/Script/Test_LidarSample.Pawn_Player|GetPrevForward _as_bp_login_pawn) (Variables|Default|GetInputForwardValue))
            (bind _output_get (Variables|/Script/Test_LidarSample.Pawn_Player|SetPrevForward _as_bp_login_pawn (Variables|Default|GetInputForwardValue)))
            (CallFunction|InputForward)))))))

(event Custom|InputRight
  ;[1 1 1] 포톤 이동 동기화 송신부
  (bind _asgm_solaseado (Utilities|Casting|CastToGM_Solaseado (Game|GetGameMode)))
  (Class|ActorSolaseadoPhoton|MovePlayerCommand (Variables|/Script/Test_LidarSample.GameModeBase_Solaseado|GetPhotonCloud _asgm_solaseado) (Variables|/Script/Test_LidarSample.Pawn_Player|GetPrevRight (Variables|Default|GetAs%20BP%20Login%20Pawn))))

(event Custom|RightGameMode1
  (params (AxisValue :type Float%20%28single-precision%29))
  (bind _returnvalue (Game|Player|GetPlayerPawn 0))
  (bind _returnvalue_2 (Transformation|GetActorRotation _returnvalue))
  (Class|Actor|AddActorWorldRotation _returnvalue (Math|Rotator|MakeRotator 0.0 0.0 (- (.yaw (Math|Rotator|Lerp(Rotator) _returnvalue_2 (Math|Conversions|RotationFromXVector (* (Math|Vector|GetRightVector (Pawn|GetControlRotation _returnvalue :!class /Script/Engine.Pawn)) AxisValue)) 0.1 true)) (.Yaw (Math|Rotator|BreakRotator _returnvalue_2))))))

(event Custom|ForwardGameMode1
  (params (AxisValue :type Float%20%28single-precision%29))
  (bind _returnvalue (Game|Player|GetPlayerPawn 0))
  (bind _returnvalue_2 (Transformation|GetActorRotation _returnvalue))
  (Class|Actor|AddActorWorldRotation _returnvalue (Math|Rotator|MakeRotator 0.0 0.0 (- (.yaw (Math|Rotator|Lerp(Rotator) _returnvalue_2 (Math|Conversions|RotationFromXVector (* (Math|Vector|GetForwardVector (Pawn|GetControlRotation _returnvalue :!class /Script/Engine.Pawn)) AxisValue)) 0.1 true)) (.Yaw (Math|Rotator|BreakRotator _returnvalue_2))))))

(event Custom|ForwardGameMode0
  (params (AxisValue :type Float%20%28single-precision%29))
  (bind _returnvalue (Game|Player|GetPlayerPawn 0))
  (bind _returnvalue_2 (Transformation|GetActorRotation _returnvalue))
  (Class|Actor|AddActorWorldRotation _returnvalue (Math|Rotator|MakeRotator 0.0 0.0 (- (.yaw (Math|Rotator|Lerp(Rotator) _returnvalue_2 (Math|Conversions|RotationFromXVector (Math|Vector|GetForwardVector (Pawn|GetControlRotation _returnvalue :!class /Script/Engine.Pawn))) 0.1 true)) (.Yaw (Math|Rotator|BreakRotator _returnvalue_2))))))

(event Custom|InputRotation
  ;[1 1 1] 회전값 서버로 송신
  (bind _asgm_solaseado (Utilities|Casting|CastToGM_Solaseado (Game|GetGameMode)))
  (Class|ActorSolaseadoPhoton|RotationPlayerX (Variables|/Script/Test_LidarSample.GameModeBase_Solaseado|GetPhotonCloud _asgm_solaseado) (Variables|Default|GetlocalYaw)))

(event Custom|moveRightKES
  (params (InputValue :type Float%20%28single-precision%29))
  (bind _as_bp_login_pawn (Variables|Default|GetAs%20BP%20Login%20Pawn))
  ;[1 1 1] 이동 입력축
  (Utilities|IsValid _as_bp_login_pawn
    (:Is%20Valid
      (Utilities|FlowControl|Sequence
        (:then_0
          (if (!= InputValue 0.0)
            (if (> InputValue 0.0)
              (Variables|Default|SetInputRightValue "Right")
              (else
                (Variables|Default|SetInputRightValue "Left")))
            (else
              (Variables|Default|SetInputRightValue "RightStop"))))
        (:then_1
          (if (Utilities|Enum|NotEqual(Enum) (Variables|/Script/Test_LidarSample.Pawn_Player|GetPrevRight _as_bp_login_pawn) (Variables|Default|GetInputRightValue))
            (bind _output_get (Variables|/Script/Test_LidarSample.Pawn_Player|SetPrevRight _as_bp_login_pawn (Variables|Default|GetInputRightValue)))
            (CallFunction|InputRight)))))))

(event Custom|moveForwardLSH
  (params (AxisValue :type Float%20%28single-precision%29))
  (bind _returnvalue (Pawn|GetControlRotation :!class /Script/Engine.Controller))
  (bind _returnvalue_2 (Math|Vector|GetForwardVector _returnvalue))
  (if (!= AxisValue 0.0)
    (Pawn|Input|AddMovementInput (Game|Player|GetPlayerPawn 0) (* (* (Math|Vector|MakeVector (.x _returnvalue_2) (.y _returnvalue_2) 0.0) AxisValue) (Variables|Default|GetmoveSpeed)) 1.0 false)
    ;[1 0.3438 0.3438] GM 카메라 세팅
    ; 1 == 연결
    ; 0 == 해제
    (bind _asgm_solaseado (Utilities|Casting|CastToGM_Solaseado (Game|GetGameMode)))
    (if (== (Variables|/Game/Project/World/GM_Solaseado.GM_Solaseado_C|GetGM_CameraSetting _asgm_solaseado) 1)
      (switch int (Variables|Default|GetCamera_MoveType)
        (:0
          (CallFunction|ForwardGameMode0 AxisValue))
        (:1
          (CallFunction|ForwardGameMode1 AxisValue))))))

(event Custom|RotationX
  (params (InputValue :type Float%20%28single-precision%29))
  ;[1 1 1] 마우스/터치 회전 입력
  (Utilities|IsValid (Variables|Default|GetAs%20BP%20Login%20Pawn)
    (:Is%20Valid
      (Utilities|FlowControl|Sequence
        (:then_0
          (Variables|Default|SetInputRotationValue (Math|Conversions|ToFloat(Integer) (Math|Float|Truncate InputValue))))
        (:then_1
          (if (!= (Variables|Default|GetlocalYaw) (Variables|Default|GetInputRotationValue))
            (bind _output_get (Variables|Default|SetlocalYaw (Variables|Default|GetInputRotationValue)))
            (CallFunction|InputRotation)))))))

(event Custom|InputForward
  ;[1 1 1] 포톤 이동 동기화 송신부
  (bind _asgm_solaseado (Utilities|Casting|CastToGM_Solaseado (Game|GetGameMode)))
  (Class|ActorSolaseadoPhoton|MovePlayerCommand (Variables|/Script/Test_LidarSample.GameModeBase_Solaseado|GetPhotonCloud _asgm_solaseado) (Variables|/Script/Test_LidarSample.Pawn_Player|GetPrevForward (Variables|Default|GetAs%20BP%20Login%20Pawn))))

(event Custom|moveRightLSH
  (params (AxisValue :type Float%20%28single-precision%29))
  (bind _returnvalue (Pawn|GetControlRotation :!class /Script/Engine.Controller))
  (bind _returnvalue_2 (Math|Vector|GetRightVector _returnvalue))
  (if (!= AxisValue 0.0)
    (Pawn|Input|AddMovementInput (Game|Player|GetPlayerPawn 0) (* (* (Math|Vector|MakeVector (.x _returnvalue_2) (.y _returnvalue_2) 0.0) AxisValue) (Variables|Default|GetmoveSpeed)) 1.0 false)
    (switch int (Variables|Default|GetCamera_MoveType)
      (:1
        (CallFunction|RightGameMode1 AxisValue)))))

(event EventBeginPlay)

(event EventTick
  (params (DeltaSeconds :type Float%20%28single-precision%29))
  (bind _returnvalue (Transformation|GetActorForwardVector))
  (bind _returnvalue_2 (Transformation|GetActorRightVector))
  (bind _self self)
  (bind _as_bp_login_pawn (Variables|Default|GetAs%20BP%20Login%20Pawn))
  (bind _as_bp_login_pawn_2 (Variables|Default|GetAs%20BP%20Login%20Pawn))
  (bind _as_bp_login_pawn_3 (Variables|Default|GetAs%20BP%20Login%20Pawn))
  (bind _returnvalue_3 (Pawn|GetControlRotation _self :!class /Script/Engine.Controller))
  (bind _fforward (Variables|/Script/Test_LidarSample.Pawn_Player|GetfForward _as_bp_login_pawn_2))
  (bind _fright (Variables|/Script/Test_LidarSample.Pawn_Player|GetfRight _as_bp_login_pawn_2))
  (bind _returnvalue_4 (* _returnvalue _fforward))
  (bind _returnvalue_5 (* _returnvalue_2 _fright))
  ;[1 1 1] 동기화에 맞춘 Tick 이동
  (Utilities|IsValid (Variables|Default|GetAs%20BP%20Login%20Pawn)
    (:Is%20Valid
      (Variables|Default|SetIsMoving false)
      (Variables|Default|SetDirectionVector "0, 0, 0")
      (Utilities|FlowControl|Sequence
        (:then_0
          (if (!= _fforward 0.0)
            (Variables|Default|SetDirectionVector (+ (Math|Vector|Normalize (Math|Vector|MakeVector (.x _returnvalue_4) (.y _returnvalue_4) 0.0)) (Variables|Default|GetDirectionVector)))
            (Variables|Default|SetIsMoving true)))
        (:then_1
          (if (!= _fright 0.0)
            (Variables|Default|SetDirectionVector (+ (Math|Vector|Normalize (Math|Vector|MakeVector (.x _returnvalue_5) (.y _returnvalue_5) 0.0)) (Variables|Default|GetDirectionVector)))
            (Variables|Default|SetIsMoving true)))
        (:then_2
          (if (Variables|Default|GetIsMoving)
            (Transformation|SetActorLocation _as_bp_login_pawn_3 (+ (* (Math|Vector|Normalize (Variables|Default|GetDirectionVector)) (* DeltaSeconds (Variables|Default|GetmoveSpeed))) (Transformation|GetActorLocation _as_bp_login_pawn_3)) false false)))
        (:then_3
          (if (!= (Variables|/Script/Test_LidarSample.Pawn_Player|GetfRotationX _as_bp_login_pawn) 0.0)
            ;;[1 1 1] 폰의 카메라 고정때문에 회전이 안돼서 컨트롤러 회전을 하였습니다.
            (Pawn|SetControlRotation (Math|Rotator|MakeRotator (.roll _returnvalue_3) (.pitch _returnvalue_3) (+ (.yaw (Transformation|GetActorRotation _as_bp_login_pawn)) (* (* (Variables|/Script/Test_LidarSample.Pawn_Player|GetfRotationX _as_bp_login_pawn) (Variables|Default|GetCamera_Rot_Speed)) (* DeltaSeconds 5e+01)))))))))))

(event Input|AxisEvents|InputAxismoveRight
  (params (AxisValue :type Float%20%28single-precision%29))
  ;[1 1 1] 이동입력축. 교체하면 됩니다.
  (CallFunction|MoveRightKES AxisValue))

(event Input|AxisEvents|InputAxismoveForward
  (params (AxisValue :type Float%20%28single-precision%29))
  ;[1 1 1] 이동입력축. 교체하면 됩니다.
  (CallFunction|MoveForwardKES AxisValue))

(event Input|AxisEvents|InputAxisMouseX
  (params (AxisValue :type Float%20%28single-precision%29))
  ;[1 1 1] 마우스로 카메라회전
  ; 마우스를 터치로 사용 세팅 => 연결 끊어놓음  ==>Touch_Input_Camera  이벤트 페이지에 touch 세팅
)

(event Input|AxisEvents|InputAxisMouseY
  (params (AxisValue :type Float%20%28single-precision%29))
  ;[1 1 1] 마우스로 카메라회전
  ; 마우스를 터치로 사용 세팅 => 연결 끊어놓음  ==>Touch_Input_Camera  이벤트 페이지에 touch 세팅
)

(event Input|AxisEvents|InputAxisMouseWheel
  (params (AxisValue :type Float%20%28single-precision%29))
  ;[1 1 1] 마우스로 카메라회전
  ; 마우스를 터치로 사용 세팅 => 연결 끊어놓음  ==>Touch_Input_Camera  이벤트 페이지에 touch 세팅
  (if (!= AxisValue 0.0)
    _))

(event Input|KeyboardEvents|Ctrl1
  (params (Key :type Key%20Structure :default "None"))
  ;[1 1 1] Test _ Seamless Level Load
  (:Pressed
    (bind _asbp_login_pawn (Utilities|Casting|CastToBP_LoginPawn (Game|Player|GetPlayerPawn 0)))
    (Default|TestTargetLength _asbp_login_pawn)))

(event Input|KeyboardEvents|K
  (params (Key :type Key%20Structure :default "None"))
  (:Pressed
    (bind _asgm_solaseado (Utilities|Casting|CastToGM_Solaseado (Game|GetGameMode)))
    (Class|ActorSolaseadoPhoton|MovePlayer (Variables|/Script/Test_LidarSample.GameModeBase_Solaseado|GetPhotonCloud _asgm_solaseado) (Transformation|GetActorLocation (Game|Player|GetPlayerPawn 0)))))

(event Input|KeyboardEvents|Ctrl3
  (params (Key :type Key%20Structure :default "None"))
  ;[1 0.1976 0.2175] Test _ Intro 스킵 후 로그인
  (:Pressed
    (bind _asbp_login_pawn (Utilities|Casting|CastToBP_LoginPawn (Game|Player|GetPlayerPawn 0)))
    (Default|LoginCustomID _asbp_login_pawn)
    (bind _asgm_solaseado (Utilities|Casting|CastToGM_Solaseado (Game|GetGameMode)))
    (Default|WidgetAllRemove _asgm_solaseado)))

(event Input|TouchEvents|InputTouch
  (params (Location :type Vector) (FingerIndex :type ETouchIndex%20Enum))
  (bind _returnvalue (Game|Player|GetPlayerPawn 0))
  (bind _returnvalue_2 (Game|Player|GetPlayerPawn 0))
  (bind _returnvalue_3 (Game|GetGameMode))
  (:Pressed
    (switch Utilities|FlowControl|Switch|SwitchonETouchIndex FingerIndex
      (:Touch1
        (bind _output_get (Variables|Default|SetFirst_Loc Location))
        (Variables|Default|SetT01_check_Rotation _output_get)
        (Variables|Default|SetFirstTouch true))
      (:Touch2
        (bind _output_get_2 (Variables|Default|SetSecond_Loc Location))
        (Variables|Default|SetStart_Distance (Math|Vector|Distance(Vector) _output_get_2 (Variables|Default|GetFirst_Loc)))
        (Variables|Default|SetT02_check_Rotation _output_get_2)
        (Variables|Default|SetSecond_Touch true)
        (if (Variables|Default|GetFirstTouch)
          (Variables|Default|SetIsZoom true)))))
  (:Released
    (bind _output_get_3 (Variables|Default|SetFirstTouch false))
    (bind _output_get_4 (Variables|Default|SetIsZoom _output_get_3))
    (Variables|Default|SetSecond_Touch _output_get_4)
    ;[1 1 1] 회전부 릴리즈 부분 추가
    (switch Utilities|FlowControl|Switch|SwitchonETouchIndex FingerIndex
      (:Touch1
        ;[1 1 1] 마우스를 땠을때 원점으로
        (CallFunction|RotationX 0.0))))
  (:Moved
    (switch Utilities|FlowControl|Switch|SwitchonETouchIndex FingerIndex
      (:Touch1
        (bind _output_get_5 (Variables|Default|SetFirst_Loc Location))
        (if (Variables|Default|GetIsZoom)
          (if (> (Math|Vector|Distance(Vector) _output_get_5 (Variables|Default|GetSecond_Loc)) (Variables|Default|GetStart_Distance))
            (bind _asbp_login_pawn (Utilities|Casting|CastToBP_LoginPawn _returnvalue_2 :!label _label))
            (bind _output_get_6 (Variables|/Script/Engine.SpringArmComponent|SetTargetArmLength (Variables|/Game/Project/Pawn/Solaseado/BP_LoginPawn.BP_LoginPawn_C|GetSpringArm _asbp_login_pawn) (Math|Float|Clamp(Float) (- (Variables|/Script/Engine.SpringArmComponent|GetTargetArmLength (Variables|/Game/Project/Pawn/Solaseado/BP_LoginPawn.BP_LoginPawn_C|GetSpringArm _asbp_login_pawn)) 1e+01) 5e+01 5e+02)))
            (bind _asgm_solaseado (Utilities|Casting|CastToGM_Solaseado _returnvalue_3))
            (Default|ChangeCamLength (Variables|/Game/Project/Widget/Chating/WB_MainMenu.WB_MainMenu_C|GetTest_PlayfabInterface (Variables|/Game/Project/World/GM_Solaseado.GM_Solaseado_C|GetWB_MainMenu _asgm_solaseado)) (Utilities|Text|ToText(Float) _output_get_6 "HalfToEven"))
            (else
              (bind _asbp_login_pawn_2 (Utilities|Casting|CastToBP_LoginPawn _returnvalue_2 :!label _label_2))
              (bind _output_get_7 (Variables|/Script/Engine.SpringArmComponent|SetTargetArmLength (Variables|/Game/Project/Pawn/Solaseado/BP_LoginPawn.BP_LoginPawn_C|GetSpringArm _asbp_login_pawn_2) (Math|Float|Clamp(Float) (+ (Variables|/Script/Engine.SpringArmComponent|GetTargetArmLength (Variables|/Game/Project/Pawn/Solaseado/BP_LoginPawn.BP_LoginPawn_C|GetSpringArm _asbp_login_pawn_2)) 1e+01) 5e+01 5e+02)))
              (bind _asgm_solaseado_2 (Utilities|Casting|CastToGM_Solaseado _returnvalue_3))
              (Default|ChangeCamLength (Variables|/Game/Project/Widget/Chating/WB_MainMenu.WB_MainMenu_C|GetTest_PlayfabInterface (Variables|/Game/Project/World/GM_Solaseado.GM_Solaseado_C|GetWB_MainMenu _asgm_solaseado_2)) (Utilities|Text|ToText(Float) _output_get_7 "HalfToEven"))))
          (else
            ;[1 1 1] 위젯 터치 -> 터치 이벤트 X -> move Event  == 잘못된 값사용
            ; ==>> 확실하게 터치이벤트가 발생할때 카메라 회전사용
            (if (Variables|Default|GetFirstTouch)
              (Pawn|Input|AddControllerPitchInput (Game|Player|GetPlayerPawn 0) (* (Variables|Default|GetCamera_Rot_Speed) (Math|Float|NormalizetoRange (- (.Y (Math|Vector|BreakVector _output_get_5)) (.y (Variables|Default|GetT01_check_Rotation))) 0.0 5e+01)))
              (CallFunction|RotationX (Math|Float|NormalizetoRange (- (.X (Math|Vector|BreakVector _output_get_5)) (.x (Variables|Default|GetT01_check_Rotation))) 0.0 5e+01))
              ;[1 1 1] 마우스 캡처로 인한 좌표문제 떄문에 테스트때 사용
              (Development|PrintString (Utilities|String|Append "X : " (Utilities|String|ToString(Float) (* (Variables|Default|GetCamera_Rot_Speed) (Math|Float|NormalizetoRange (- (.X (Math|Vector|BreakVector _output_get_5)) (.x (Variables|Default|GetT01_check_Rotation))) 0.0 5e+01))) ", Y : " (Utilities|String|ToString(Float) (* (Variables|Default|GetCamera_Rot_Speed) (Math|Float|NormalizetoRange (- (.Y (Math|Vector|BreakVector _output_get_5)) (.y (Variables|Default|GetT01_check_Rotation))) 0.0 5e+01)))))))))
      (:Touch2
        (bind _output_get_8 (Variables|Default|SetSecond_Loc Location))
        (if (Variables|Default|GetIsZoom)
          (if (> (Math|Vector|Distance(Vector) _output_get_8 (Variables|Default|GetFirst_Loc)) (Variables|Default|GetStart_Distance))
            (goto _label)
            (else
              (goto _label_2)))
          (elif (Variables|Default|GetSecond_Touch)
            (Pawn|Input|AddControllerYawInput _returnvalue (* (Variables|Default|GetCamera_Rot_Speed) (Math|Float|NormalizetoRange (- (.X (Math|Vector|BreakVector _output_get_8)) (.x (Variables|Default|GetT02_check_Rotation))) 0.0 5e+01)))
            (Pawn|Input|AddControllerPitchInput _returnvalue (* (Variables|Default|GetCamera_Rot_Speed) (Math|Float|NormalizetoRange (- (.Y (Math|Vector|BreakVector _output_get_8)) (.y (Variables|Default|GetT02_check_Rotation))) 0.0 5e+01)))))))))

(fn ConstructionScript)