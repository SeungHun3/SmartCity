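; Test game mode for the SimPoly world that streams numbered sublevels laid out as a row/column grid.
; A level change unloads the previous neighbours except the new level, then loads it and its four orthogonal neighbours.
; Loads and unloads chain one at a time through pending arrays, updating PC_SimPoly's test icons.
; An event toggles player culling, while FPS-triggered culling and Photon login logic are disconnected.
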(event Custom|LoadLevel_SimPoly
  (params (Level :type String))
  ;[1 1 1] Call Load Level
  (Variables|Default|SetNextLevel Level)
  (CallFunction|CheckOutsideUnloadLevel)
  ;[1 1 1] 주변 레벨 추가 로드 목록
  (CallFunction|CheckOutsideLoadLevel)
  (CallFunction|LoadLevel (Variables|Default|GetCurrentLevel)))

(event Custom|UnloadLevel_OutsideSimpoly
  (params (Level :type String))
  (bind _returnvalue (Utilities|String|Append "SimPoly" Level))
  (bind _outsideunloadlevel (Variables|Default|GetOutsideUnloadLevel))
  ;[1 1 1] Call Unload Level
  (Game|UnloadStreamLevel(byName) (Utilities|String|StringToName _returnvalue) false)
  (bind _aspc_sim_poly (Utilities|Casting|CastToPC_SimPoly (Game|GetPlayerController 0)))
  (Default|TestCheckIcon _aspc_sim_poly _returnvalue false)
  (bind _array_element (Utilities|Array|ForEachLoopwithBreak _outsideunloadlevel :!label _label)
    (:LoopBody
      (CallFunction|UnloadLevelOutsideSimpoly _array_element)
      (Development|PrintString (Utilities|String|Append "// test _ Check Outside Unload Level :: " _array_element))
      (Utilities|Array|RemoveItem _outsideunloadlevel _array_element)
      (goto _label Break))))

(event Custom|Reset_FPSCulling
  (Utilities|FlowControl|DoOnce false) ; enters at Reset
)

(event Custom|LoadLevel
  (params (Level :type String))
  (bind _returnvalue (Utilities|String|Append "SimPoly" Level))
  (bind _outsideloadlevel (Variables|Default|GetOutsideLoadLevel))
  ;[1 1 1] Load Stream Level & Test Widget
  (Game|LoadStreamLevel(byName) (Utilities|String|StringToName _returnvalue) true)
  (Development|PrintString (Utilities|String|Append "// Load Stream Level :: " _returnvalue))
  (bind _aspc_sim_poly (Utilities|Casting|CastToPC_SimPoly (Game|GetPlayerController 0)))
  (Default|TestCheckIcon _aspc_sim_poly _returnvalue true)
  ;[1 1 1] 이웃 레벨 추가 로드
  (bind (_array_element _array_index) (Utilities|Array|ForEachLoopwithBreak _outsideloadlevel :!label _label)
    (:LoopBody
      (CallFunction|LoadLevel _array_element)
      (Utilities|Array|RemoveIndex _outsideloadlevel _array_index)
      (goto _label Break))))

(event EventTick
  (params (DeltaSeconds :type Float%20%28single-precision%29)))

(event EventBeginPlay)

(fn ConstructionScript)

(fn CurrentLevelRow
  (return (/ (- (Math|Conversions|ToInteger(Byte) (Variables|Default|GetCurrentLevel)) 1) (Variables|Default|GetMaxCol))))

(fn CurrentLevelCol
  (return (Math|Integer|%(Integer) (- (Math|Conversions|ToInteger(Byte) (Variables|Default|GetCurrentLevel)) 1) (Variables|Default|GetMaxCol))))

(fn CheckOutsideLoadLevel
  (bind _row (CallFunction|CurrentLevelRow))
  (bind _col (CallFunction|CurrentLevelCol))
  (bind _outsideloadlevel (Variables|Default|GetOutsideLoadLevel))
  (bind _returnvalue (- _row 1))
  (bind _returnvalue_2 (- _col 1))
  (bind _returnvalue_3 (+ _row 1))
  (bind _returnvalue_4 (+ _col 1))
  (Utilities|Array|Clear (Variables|Default|GetOutsideLoadLevel))
  (Utilities|FlowControl|Sequence
    (:then_0
      (LocalVariables|SetCheckIndex _returnvalue_3)
      (if (< _returnvalue_3 (Variables|Default|GetMaxRow))
        ;[1 1 1] 로드 가능한 레벨 체크
        (Utilities|Array|Add _outsideloadlevel (Utilities|String|ToString(Integer) (+ (+ (* (LocalVariables|GetCheckIndex) (Variables|Default|GetMaxCol)) (CallFunction|CurrentLevelCol)) 1)) :!label _label)
        (Variables|Default|SetTest_OutsideLoadLevel _outsideloadlevel :!label _label_2)))
    (:then_1
      (LocalVariables|SetCheckIndex _returnvalue)
      (if (>= _returnvalue 0)
        (goto _label)))
    (:then_2
      (LocalVariables|SetCheckIndex _returnvalue_4)
      (if (< _returnvalue_4 (Variables|Default|GetMaxCol))
        (Utilities|Array|Add _outsideloadlevel (Utilities|String|ToString(Integer) (+ (+ (* (CallFunction|CurrentLevelRow) (Variables|Default|GetMaxCol)) (LocalVariables|GetCheckIndex)) 1)) :!label _label_3)
        (goto _label_2)))
    (:then_3
      (LocalVariables|SetCheckIndex _returnvalue_2)
      (if (>= _returnvalue_2 0)
        (goto _label_3)))))

(fn CheckOutsideUnloadLevel
  (bind _outsideunloadlevel (Variables|Default|GetOutsideUnloadLevel))
  (Utilities|Array|Clear (Variables|Default|GetOutsideUnloadLevel))
  (for _array_element (Variables|Default|GetTest_OutsideLoadLevel)
    (if (Utilities|Enum|NotEqual(Enum) (Variables|Default|GetNextLevel) _array_element)
      (Utilities|Array|Add (Variables|Default|GetOutsideUnloadLevel) _array_element)))
  (Utilities|Array|Clear (Variables|Default|GetTest_OutsideLoadLevel))
  (LocalVariables|SetFirstUnloadLevel (Utilities|Array|Get(acopy) _outsideunloadlevel))
  (Utilities|Array|RemoveIndex _outsideunloadlevel)
  (CallFunction|UnloadLevelOutsideSimpoly (LocalVariables|GetFirstUnloadLevel))
  (Variables|Default|SetCurrentLevel (Variables|Default|GetNextLevel))
  (return))

(fn GetFPS
  (return (Variables|Default|GetFps)))