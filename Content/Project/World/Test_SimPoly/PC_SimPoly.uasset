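; Test player controller for the SimPoly test world that shows the Solaseado login widget and provides debug controls.
; Input cycles walk speed, toggles the cursor, rotates the camera and zooms the spring arm, shifting message box and name tag with it.
; Test events reset location to a tagged PlayerStart and spawn or clear counted NPC pawns.
; Level-streaming widget creation, player character caching and the map-load check are disconnected, though active logic uses those references.
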(event Custom|Test_CheckIcon
  (params (LevelName :type String) (isLoadLevel :type Boolean))
  ;[1 1 1] Test _ load Map Checker
  ; / 테스트 기능 / 로드 맵 체커
)

(event Custom|Test_SpawnNPC
  (bind _returnvalue (Game|Player|GetPlayerPawn 0))
  (bind _testpawnlist (Variables|Default|GetTestPawnlist))
  ;[1 1 1] Test _ NPC 스폰
  (bind _returnvalue_2 (Game|SpawnActorfromClass "/Game/Project/Pawn/TestPawn_npc.TestPawn_npc_C" (Math|Transform|MakeTransform (+ (* (Transformation|GetActorForwardVector _returnvalue) 1e+02) (Transformation|GetActorLocation _returnvalue)) "0, 0, 0" "1,1,1") "AlwaysSpawn" 0 false 0))
  ;[1 1 1] 위젯 카운터 표시
  (Utilities|Array|Add _testpawnlist _returnvalue_2)
  (Default|TestSpawnCnt (Variables|Default|GetWidget_LevelStream) (Utilities|Text|ToText(Integer) (Utilities|Array|Length _testpawnlist))))

(event Custom|Test_RemoveSpawnNPC
  (bind _testpawnlist (Variables|Default|GetTestPawnlist))
  ;[1 1 1] Test_NPC Remove
  (Actor|DestroyActor _testpawnlist)
  (Utilities|Array|Clear _testpawnlist))

(event Custom|Test_SpeedChanger
  (bind _as_bp_player_character (Variables|Default|GetAs%20BP%20Player%20Character))
  ;[1 1 1] Test Speed Change
  (Utilities|FlowControl|MultiGate false true -1
    (:Out%200
      (Development|PrintString "// Test Player Speed Change 0 :: 200")
      (Default|SetMaxWalkSpeed _as_bp_player_character 2e+02))
    (:Out%201
      (Development|PrintString "// Test Player Speed Change 1 :: 400")
      (Default|SetMaxWalkSpeed _as_bp_player_character 4e+02))
    (:Out%202
      (Development|PrintString "// Test Player Speed Change 2 :: 800")
      (Default|SetMaxWalkSpeed _as_bp_player_character 8e+02))
    (:Out%203
      (Development|PrintString "// Test Player Speed Change 3 :: 1600")
      (Default|SetMaxWalkSpeed _as_bp_player_character 1.6e+03))))

(event Custom|Test_LocationReset
  (bind _outactors (Actor|GetAllActorsOfClasswithTag "/Script/Engine.PlayerStart" "Test"))
  (Utilities|IsValid (Utilities|Array|Get(acopy) _outactors)
    (:Is%20Valid
      (Transformation|SetActorLocation (Pawn|GetControlledPawn (Game|GetPlayerController 0)) (Transformation|GetActorLocation (Utilities|Array|Get(acopy) _outactors)) false false))))

(event EventBeginPlay
  ;[1 1 1] Login Widget -> Add Viewport
  (bind _returnvalue (UserInterface|CreateWidget "/Game/Project/Widget/WB_SolaseadoLogin.WB_SolaseadoLogin_C"))
  (bind _output_get (Variables|Default|SetWidget_SolaseadpLogin _returnvalue))
  (UserInterface|Viewport|AddtoViewport _output_get 0))

(event Input|AxisEvents|InputAxisMouseX
  (params (AxisValue :type Float%20%28single-precision%29))
  (bind _as_bp_player_character (Variables|Default|GetAs%20BP%20Player%20Character))
  ;[0 0.009347 1] 카메라 회전
  (if (!= AxisValue 0.0)
    (Utilities|IsValid _as_bp_player_character
      (:Is%20Valid
        (Default|SetCameraRotationYaw _as_bp_player_character AxisValue)))))

(event Input|AxisEvents|InputAxisMouseWheel
  (params (AxisValue :type Float%20%28single-precision%29))
  (bind _as_bp_player_character (Variables|Default|GetAs%20BP%20Player%20Character))
  (bind _messagebox (Variables|/Script/Test_LidarSample.Character_Player|GetMessageBox _as_bp_player_character))
  (bind _nametag (Variables|/Game/Project/Pawn/BP_PlayerCharacter.BP_PlayerCharacter_C|GetNameTag _as_bp_player_character))
  (bind _springarmcomp (Variables|/Script/Test_LidarSample.Character_Player|GetSpringArmComp _as_bp_player_character))
  (bind _relativelocation (Variables|/Script/Engine.SceneComponent|GetRelativeLocation _messagebox))
  (bind _relativelocation_2 (Variables|/Script/Engine.SceneComponent|GetRelativeLocation _nametag))
  ;[0 0.009347 1] 마우스 휠 // 카메라 줌인 아웃
  (if (!= AxisValue 0.0)
    (bind _output_get (Variables|/Script/Engine.SpringArmComponent|SetTargetArmLength _springarmcomp (Math|Float|Clamp(Float) (+ (Variables|/Script/Engine.SpringArmComponent|GetTargetArmLength _springarmcomp) (* AxisValue -1e+01)) 0.0 5e+02)))
    (Transformation|SetRelativeLocation _messagebox (Math|Vector|MakeVector _output_get (.y _relativelocation) (.z _relativelocation)) false false)
    (Transformation|SetRelativeLocation _nametag (Math|Vector|MakeVector _output_get (.y _relativelocation_2) (.z _relativelocation_2)) false false)))

(event Input|AxisEvents|InputAxisMouseY
  (params (AxisValue :type Float%20%28single-precision%29))
  (bind _as_bp_player_character (Variables|Default|GetAs%20BP%20Player%20Character))
  ;[0 0.009347 1] 카메라 회전
  (if (!= AxisValue 0.0)
    (Utilities|IsValid _as_bp_player_character
      (:Is%20Valid
        (Default|SetCameraRotationPitch _as_bp_player_character AxisValue)))))

(event Input|KeyboardEvents|LeftCtrl
  (params (Key :type Key%20Structure :default "None"))
  (:Pressed
    (Variables|Default|SetbShowMouseCursor (not (Variables|Default|GetbShowMouseCursor)))))

(event Input|KeyboardEvents|Ctrl1
  (params (Key :type Key%20Structure :default "None"))
  (:Pressed
    (Development|PrintString "// Test _ Check Spawn Char")
    (CallFunction|TestSpawnNPC)))

(event Input|KeyboardEvents|Ctrl2
  (params (Key :type Key%20Structure :default "None"))
  (:Pressed
    (Development|PrintString "// Test _ Check Remove Spawn Char")
    (CallFunction|TestRemoveSpawnNPC)))

(event Input|KeyboardEvents|LeftShift
  (params (Key :type Key%20Structure :default "None"))
  (bind _as_bp_player_character (Variables|Default|GetAs%20BP%20Player%20Character))
  ;[1 1 1] Test Speed Change
  (:Pressed
    (Utilities|FlowControl|MultiGate false true -1
      (:Out%200
        (Development|PrintString "// Test Player Speed Change 0 :: 200")
        (Default|SetMaxWalkSpeed _as_bp_player_character 2e+02))
      (:Out%201
        (Development|PrintString "// Test Player Speed Change 1 :: 400")
        (Default|SetMaxWalkSpeed _as_bp_player_character 4e+02))
      (:Out%202
        (Development|PrintString "// Test Player Speed Change 2 :: 800")
        (Default|SetMaxWalkSpeed _as_bp_player_character 8e+02))
      (:Out%203
        (Development|PrintString "// Test Player Speed Change 3 :: 1600")
        (Default|SetMaxWalkSpeed _as_bp_player_character 1.6e+03)))))

(fn ConstructionScript)