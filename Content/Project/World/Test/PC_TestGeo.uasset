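; Test player controller for trying out geographic coordinate conversions in a level.
; On BeginPlay it creates the UMG_GeoStatusBar widget and adds it to the viewport.
; Debug keys Alt+1 to Alt+3 print a test message, cast the game mode to GM_TestGeo and call its world-to-geo, engine-to-projected and engine-to-geographic functions respectively.
; The conversion logic lives in the game mode.
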(event EventBeginPlay
  (bind _returnvalue (UserInterface|CreateWidget "/GeoReferencing/UI/UMG_GeoStatusBar.UMG_GeoStatusBar_C"))
  (UserInterface|Viewport|AddtoViewport _returnvalue 0))

(event Input|KeyboardEvents|Alt1
  (params (Key :type Key%20Structure :default "None"))
  ;[1 1 1] 코멘트
  (:Pressed
    (Development|PrintString "// Test _ Geo Location")
    (bind _asgm_test_geo (Utilities|Casting|CastToGM_TestGeo (Game|GetGameMode)))
    (Default|GeoWorldtoGeo _asgm_test_geo)))

(event Input|KeyboardEvents|Alt2
  (params (Key :type Key%20Structure :default "None"))
  (:Pressed
    (Development|PrintString "// Test _ Geo Location")
    (bind _asgm_test_geo (Utilities|Casting|CastToGM_TestGeo (Game|GetGameMode)))
    (Default|GeoEnginetoProjected _asgm_test_geo)))

(event Input|KeyboardEvents|Alt3
  (params (Key :type Key%20Structure :default "None"))
  (:Pressed
    (Development|PrintString "// Test _ Geo Location")
    (bind _asgm_test_geo (Utilities|Casting|CastToGM_TestGeo (Game|GetGameMode)))
    (Default|GeoEnginetoGeographic _asgm_test_geo)))

(fn ConstructionScript)