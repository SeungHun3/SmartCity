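; GM_TestGeo is a test Blueprint that prints the player pawn's location converted into geospatial coordinates.
; Three custom events compare routes: a direct world-to-geo lookup, and GeoReferencingSystem conversions from engine space to projected (via ECEF) or to geographic (via projected).
; Each prints its result on screen, though the geographic output reuses the "Ecef to projected" label.
; An unconnected print holds reference coordinates for Haenam.
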(event Custom|Geo_WorldToGeo
  (bind (_longitude _latitude _altitude _error) (|GetGeoLocationatWorldPosition (Transformation|GetActorLocation (Game|Player|GetPlayerPawn 0)))
    (:OnSuccess
      (Development|PrintString (Utilities|String|Append "Longitude :: " (Utilities|String|ToString(Float) _longitude) " / Latitude::" (Utilities|String|ToString(Float) _latitude) "/ Altitude :: " (Utilities|String|ToString(Float) _altitude) "/ Error :: " _error)))))

(event Custom|Geo_EngineToProjected
  (bind _returnvalue (Class|GeoReferencingSystem|GetGeoReferencingSystem))
  (bind _ecefcoordinates (Class|GeoReferencingSystem|EnginetoECEF _returnvalue (Transformation|GetActorLocation (Game|Player|GetPlayerPawn 0))))
  (bind _projectedcoordinates (Class|GeoReferencingSystem|ECEFtoProjected _returnvalue _ecefcoordinates))
  (Development|PrintString (Utilities|String|Append "// Ecef to projected :: " " x :: " (Utilities|String|ToString(Float) (.OutX (Class|CartesianCoordinatesFunctionLibrary|ToFloatApproximation _projectedcoordinates))) " y :: " (Utilities|String|ToString(Float) (.OutY (Class|CartesianCoordinatesFunctionLibrary|ToFloatApproximation _projectedcoordinates))) " z :: " (Utilities|String|ToString(Float) (.OutZ (Class|CartesianCoordinatesFunctionLibrary|ToFloatApproximation _projectedcoordinates))))))

(event Custom|Geo_EngineToGeographic
  (bind _returnvalue (Class|GeoReferencingSystem|GetGeoReferencingSystem))
  (bind _projectedcoordinates (Class|GeoReferencingSystem|EnginetoProjected _returnvalue (Transformation|GetActorLocation (Game|Player|GetPlayerPawn 0))))
  (bind _geographiccoordinates (Class|GeoReferencingSystem|ProjectedtoGeographic _returnvalue _projectedcoordinates))
  (Development|PrintString (Utilities|String|Append "// Ecef to projected :: " " Latitude :: " (Utilities|String|ToString(Float) (.OutLatitude (Class|GeographicCoordinatesFunctionLibrary|ToFloatApproximation _geographiccoordinates))) " Longitude :: " (Utilities|String|ToString(Float) (.OutLongitude (Class|GeographicCoordinatesFunctionLibrary|ToFloatApproximation _geographiccoordinates))) " Altitude :: " (Utilities|String|ToString(Float) (.OutAltitude (Class|GeographicCoordinatesFunctionLibrary|ToFloatApproximation _geographiccoordinates))))))

(fn ConstructionScript)