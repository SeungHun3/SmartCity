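; BP_GM is a game-mode-style world Blueprint that starts the Photon multiplayer session for what appears to be a virtual guide project.
; On BeginPlay it spawns a BP_Photon actor at the origin, stores it as PhotonClient and logs in under a "Virtual Guide" name with a random numeric suffix.
; It also shows the mouse cursor and turns on FPS and unit stat overlays for performance testing.
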(event EventBeginPlay
  (Utilities|FlowControl|Sequence
    (:then_0
      (bind _returnvalue (Game|SpawnActorfromClass "/Game/Project/Actor/BP_Photon.BP_Photon_C" (Math|Transform|MakeTransform "0, 0, 0") "AlwaysSpawn" 0 0))
      (bind _output_get (Variables|Default|SetPhotonClient _returnvalue))
      (Class|ActorPhoton|ConnectLogin _output_get (Utilities|String|Append "Virtual Guide" (Utilities|String|ToString(Integer) (Math|Random|RandomInteger 99))))
      (Variables|/Script/Engine.PlayerController|SetbShowMouseCursor (Game|GetPlayerController 0) true))
    (:then_1
      ;[1 1 1] 스펙 테스트 커멘트
      (Development|ExecuteConsoleCommand "stat fps" 0)
      (Development|ExecuteConsoleCommand "stat unit" 0))))

(fn ConstructionScript)